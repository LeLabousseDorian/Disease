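; Light manager Blueprint that generates recurring, randomized lightning flashes as an intensity value.
; From BeginPlay, a self-restarting Lightning event waits a random time within the LightningTiming range, then picks one of three timeline curves.
; The timeline writes the chosen curve to LightningIntencity each update and schedules the next flash when finished; this graph does not apply that value to any light.
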(event Custom|Lightning
  (bind _lightning_timing (Variables|Default|GetLightning_Timing))
  (bind (_x _y) (Math|Vector2D|BreakVector2D _lightning_timing))
  (Utilities|FlowControl|Delay (Math|Random|RandomFloatinRange _x _y))
  (Variables|Default|SetRand_Lightning (Math|Random|RandomIntegerinRange 0 2))
  (bind (_direction _lightning_1 _lightning_2 _lightning_3) (Timeline|Timeline_Lightnings PlayFromStart)
    (:Update
      (Variables|Default|SetLightning_Intencity (Utilities|Select :Index (Variables|Default|GetRand_Lightning) :Option%200 _lightning_1 :Option%201 _lightning_2 :Option%202 _lightning_3)))
    (:Finished
      (CallFunction|Lightning))))

(event EventBeginPlay
  (CallFunction|Lightning))

(fn ConstructionScript)