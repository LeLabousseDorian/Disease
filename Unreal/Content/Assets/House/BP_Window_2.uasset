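; BP_Window_2 is a house window actor that lets outside lightning and night light shine in through two spot lights.
; On BeginPlay it caches the first BP_Light_Manager found in the level.
; Every Tick it copies the manager's LightningIntencity and NightLight values to the intensities of the lightning and night spot lights.
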(event EventTick
  (params (DeltaSeconds :type Float%20%28single-precision%29))
  (Rendering|Components|Light|SetIntensity (Variables|Default|GetLightning_SpotLight) (Variables|/Game/Assets/House/BP_Light_Manager.BP_Light_Manager_C|GetLightning_Intencity (Variables|Default|GetLight_Manager)))
  (Rendering|Components|Light|SetIntensity (Variables|Default|GetNight_SpotLight) (Variables|/Game/Assets/House/BP_Light_Manager.BP_Light_Manager_C|GetNight_Light (Variables|Default|GetLight_Manager))))

(event EventBeginPlay
  (bind _outactors (Actor|GetAllActorsOfClass "/Game/Assets/House/BP_Light_Manager.BP_Light_Manager_C"))
  (Variables|Default|SetLight_Manager (Utilities|Array|Get(acopy) _outactors)))

(fn ConstructionScript)