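; BP_Lampe_Murale is a wall lamp actor with a point light and a spot light that follow a global on/off state.
; On BeginPlay it caches the first BP_Light_Manager found in the level.
; Every Tick it polls the manager's LightOn flag and sets both light intensities to fixed lit values or zero, rather than reacting to a change event.
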(event EventTick
  (params (DeltaSeconds :type Float%20%28single-precision%29))
  (if (Variables|/Game/Assets/House/BP_Light_Manager.BP_Light_Manager_C|GetLight_On (Variables|Default|GetLight_Manager))
    (Rendering|Components|Light|SetIntensity (Variables|Default|GetPointLight) 5e+01)
    (Rendering|Components|Light|SetIntensity (Variables|Default|GetSpotLight) 2.5e+02)
    (else
      (Rendering|Components|Light|SetIntensity (Variables|Default|GetPointLight) 0.0)
      (Rendering|Components|Light|SetIntensity (Variables|Default|GetSpotLight) 0.0))))

(event EventBeginPlay
  (bind _outactors (Actor|GetAllActorsOfClass "/Game/Assets/House/BP_Light_Manager.BP_Light_Manager_C"))
  (Variables|Default|SetLight_Manager (Utilities|Array|Get(acopy) _outactors)))

(fn ConstructionScript)