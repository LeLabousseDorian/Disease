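; BP_Disjoncteur is an interactable circuit breaker with a lever that switches the level lighting on and off.
; Each interaction alternates state through a FlipFlop, driving a timeline that rotates the lever forward or back.
; When the lever finishes switching on, the breaker material changes, the level's BP_Light_Manager gets LightOn set and an assigned level sequence plays.
; Switching off updates the material and manager immediately, then reverses the lever.
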(event EventOnInteract
  (params (Player :type BP%20Player%20Object%20Reference))
  (Utilities|FlowControl|FlipFlop
    (:A
      (Variables|Default|SetLight_On true)
      (bind _newtrack_0 (Timeline|Timeline_0 Play)
        (:Update
          (Transformation|SetRelativeRotation (Variables|Default|GetLever) (Math|Rotator|Lerp(Rotator) "0.000000,-90.000000,95.000000" "0.000000,-90.000000,-20.000000" _newtrack_0 true) false false))
        (:Finished
          (if (Variables|Default|GetLight_On)
            (Rendering|Material|SetMaterial (Variables|Default|GetDisjoncteur) 4 "/Game/Assets/Disjoncteur/Materials/Disjoncteur_ON_M.Disjoncteur_ON_M")
            (Variables|/Game/Blueprints/Actors/Actor_LD/BP_Light_Manager.BP_Light_Manager_C|SetLight_On (Variables|Default|GetLight_Manager) true)
            (Sequencer|Player|Play (Variables|/Script/LevelSequence.LevelSequenceActor|GetSequencePlayer (Variables|Default|GetSequence%20To%20Launch)) :!class /Script/MovieScene.MovieSceneSequencePlayer)))))
    (:B
      (Variables|Default|SetLight_On false)
      (Rendering|Material|SetMaterial (Variables|Default|GetDisjoncteur) 4 "/Game/Assets/Disjoncteur/Materials/Disjoncteur_OFF_M.Disjoncteur_OFF_M")
      (Variables|/Game/Blueprints/Actors/Actor_LD/BP_Light_Manager.BP_Light_Manager_C|SetLight_On (Variables|Default|GetLight_Manager) false)
      (Timeline|Timeline_0 Reverse))))

(event EventBeginPlay
  ;[1 1 1] Ref au Light_Manager
  (bind _outactors (Actor|GetAllActorsOfClass "/Game/Blueprints/Actors/Actor_LD/BP_Light_Manager.BP_Light_Manager_C"))
  (Variables|Default|SetLight_Manager (Utilities|Array|Get(acopy) _outactors)))

(fn ConstructionScript)