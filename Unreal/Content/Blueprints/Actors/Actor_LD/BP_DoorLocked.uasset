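; BP_DoorLocked is a lockable door actor that players open and close by interacting.
; OnInteract asks the BPSCDoor component whether the player's inventory allows opening, then a FlipFlop plays or reverses a timeline that lerps the mesh's relative rotation.
; CloseDoor re-triggers the same FlipFlop only when its state indicates the door is open.
; OnOpenLocked exposes the inventory check as a return value.
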(event Custom|CloseDoor
  (if (stale _isa)
    (bind _isa (Utilities|FlowControl|FlipFlop)
      (:A
        (bind _newtrack_0 (Timeline|Timeline_0 Play)
          (:Update
            (Transformation|SetRelativeRotation (Variables|Default|GetStaticMesh) (Math|Rotator|Lerp(Rotator) "0, 0, 0" "0,90.000000, 0" _newtrack_0 true) false false))))
      (:B
        (Timeline|Timeline_0 Reverse)))))

(event EventOnInteract
  (params (Player :type BP%20Player%20Object%20Reference))
  (bind _canopen (Default|CanOpen (Variables|Default|GetBP_SC_Door) (Variables|/Game/Blueprints/Player/BP_Player.BP_Player_C|GetInventory Player)))
  (if _canopen
    (bind _isa (Utilities|FlowControl|FlipFlop)
      (:A
        (bind _newtrack_0 (Timeline|Timeline_0 Play)
          (:Update
            (Transformation|SetRelativeRotation (Variables|Default|GetStaticMesh) (Math|Rotator|Lerp(Rotator) "0, 0, 0" "0,90.000000, 0" _newtrack_0 true) false false))))
      (:B
        (Timeline|Timeline_0 Reverse)))))

(fn ConstructionScript)

(fn OnOpenLocked
  (params (Player :type BP%20Player%20Object%20Reference))
  (bind _canopen (Default|CanOpen (Variables|Default|GetBP_SC_Door) (Variables|/Game/Blueprints/Player/BP_Player.BP_Player_C|GetInventory Player)))
  (return _canopen))