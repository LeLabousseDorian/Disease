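; BP_Lampe_Murale is a wall lamp actor that switches on and off with the level's light manager.
; On BeginPlay it caches the first BP_Light_Manager found in the level.
; Every Tick it polls that manager's LightOn flag, setting point and spot light intensities and swapping the mesh's second material slot between lit and unlit materials.
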(event EventTick
  (params (DeltaSeconds :type Float%20%28single-precision%29))
  (if (Variables|/Game/Blueprints/Actors/Actor_LD/BP_Light_Manager.BP_Light_Manager_C|GetLight_On (Variables|Default|GetLight_Manager))
    (Rendering|Components|Light|SetIntensity (Variables|Default|GetPointLight) 5e+01)
    (Rendering|Components|Light|SetIntensity (Variables|Default|GetSpotLight) 2.5e+02)
    (Rendering|Material|SetMaterial (Variables|Default|GetStaticMesh) 1 "/Game/Assets/Lamps/Lampe_Light_ON.Lampe_Light_ON")
    (else
      (Rendering|Components|Light|SetIntensity (Variables|Default|GetPointLight) 0.0)
      (Rendering|Components|Light|SetIntensity (Variables|Default|GetSpotLight) 0.0)
      (Rendering|Material|SetMaterial (Variables|Default|GetStaticMesh) 1 "/Game/Assets/Lamps/Lampe_Light_OFF.Lampe_Light_OFF"))))

(event EventBeginPlay
  (bind _outactors (Actor|GetAllActorsOfClass "/Game/Blueprints/Actors/Actor_LD/BP_Light_Manager.BP_Light_Manager_C"))
  (Variables|Default|SetLight_Manager (Utilities|Array|Get(acopy) _outactors)))

(fn ConstructionScript)