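; Storm manager actor that drives rain audio and random lightning strikes with delayed thunder.
; Unless Debug is set, a looping routine from BeginPlay sets rain volume and fires lightning at random intervals.
; Each strike writes one of three random timeline curves to LightningIntencity, then plays thunder after a random delay.
; A box overlap by a component named "CollisionCylinder" also triggers a strike.
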(event OnComponentBeginOverlap(Box)
  (params (OverlappedComponent :type Primitive%20Component%20Object%20Reference) (OtherActor :type Actor%20Object%20Reference) (OtherComp :type Primitive%20Component%20Object%20Reference) (OtherBodyIndex :type Integer) (bFromSweep :type Boolean) (SweepResult :type Hit%20Result%20Structure%20%28by%20ref%29))
  ;[1 1 1] Collider
  (if (Utilities|Enum|Equal(Enum) (Utilities|GetObjectName OtherComp) "CollisionCylinder")
    (CallFunction|Lightning)))

(event Custom|Lightning
  (bind _thunder_timing (Variables|Lightning|GetThunder_Timing))
  (bind (_x _y) (Math|Vector2D|BreakVector2D _thunder_timing))
  ;[1 1 1] Lightning + Thunder
  (Variables|Lightning|SetRand_Lightning (Math|Random|RandomIntegerinRange 0 2))
  (bind (_direction _lightning_1 _lightning_2 _lightning_3) (Timeline|Timeline_Lightnings PlayFromStart)
    (:Update
      (Variables|Lightning|SetLightning_Intencity (Utilities|Select :Index (Variables|Lightning|GetRand_Lightning) :Option%200 _lightning_1 :Option%201 _lightning_2 :Option%202 _lightning_3)))
    (:Finished
      (Utilities|FlowControl|Delay (Math|Random|RandomFloatinRange _x _y))
      (Audio|Components|Audio|SetVolumeMultiplier (Variables|Default|GetThunder_Audio) (Variables|Sound|GetThunder_Volume) :!class /Script/Engine.AudioComponent)
      (Audio|Components|Audio|Play (Variables|Default|GetThunder_Audio) 0.0))))

(event Custom|Lightning_Routine
  (bind _lightning_timing (Variables|Lightning|GetLightning_Timing))
  (bind (_x _y) (Math|Vector2D|BreakVector2D _lightning_timing))
  ;[1 1 1] Boucle Lightning
  ;;[1 1 1] Rain volume
  (Audio|Components|Audio|SetVolumeMultiplier (Variables|Default|GetRain_Audio) (Variables|Sound|GetRain_Volume) :!class /Script/Engine.AudioComponent)
  (Utilities|FlowControl|Delay (Math|Random|RandomFloatinRange _x _y))
  (CallFunction|Lightning)
  (CallFunction|LightningRoutine))

(event EventBeginPlay
  ;[1 1 1] BeginPlay
  (Audio|Components|Audio|Stop (Variables|Default|GetThunder_Audio))
  (if (not (Variables|Default|GetDebug))
    (CallFunction|LightningRoutine)))

(fn ConstructionScript)