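; BP_Window is a level-design window actor with a configurable mesh that reflects the scene's lightning, night light and rain.
; On BeginPlay it caches the first BP_Light_Manager found in the level.
; Each Tick it copies that manager's values to the intensity of its lightning and night spot lights and to its rain audio volume.
; The construction script applies the Mesh variable to the static mesh component.
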(event EventTick
  (params (DeltaSeconds :type Float%20%28single-precision%29))
  ;[1 1 1] Gestion de l'intencité
  (Rendering|Components|Light|SetIntensity (Variables|Default|GetLightning_SpotLight) (Variables|/Game/Blueprints/Actors/Actor_LD/BP_Light_Manager.BP_Light_Manager_C|GetLightning_Intencity (Variables|Default|GetLight_Manager)))
  (Rendering|Components|Light|SetIntensity (Variables|Default|GetNight_SpotLight) (Variables|/Game/Blueprints/Actors/Actor_LD/BP_Light_Manager.BP_Light_Manager_C|GetNight_Light (Variables|Default|GetLight_Manager)))
  (Audio|Components|Audio|SetVolumeMultiplier (Variables|Default|GetRain_02_Audio) (Variables|/Game/Blueprints/Actors/Actor_LD/BP_Light_Manager.BP_Light_Manager_C|GetRain_Volume (Variables|Default|GetLight_Manager)) :!class /Script/Engine.AudioComponent))

(event EventBeginPlay
  ;[1 1 1] Ref au Light_Manager
  (bind _outactors (Actor|GetAllActorsOfClass "/Game/Blueprints/Actors/Actor_LD/BP_Light_Manager.BP_Light_Manager_C"))
  (Variables|Default|SetLight_Manager (Utilities|Array|Get(acopy) _outactors)))

(fn ConstructionScript
  (Components|StaticMesh|SetStaticMesh (Variables|Default|GetStaticMesh) (Variables|Default|GetMesh)))