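; BP_Chair is a chair the player can push or get onto by interacting.
; Pushing sets the player's walk speed to their pushing speed, and dropping restores the base speed.
; Interacting unbinds look and movement, then a timeline lerps the player capsule to the standing position on the chair without sweeping.
; Movement is rebound on each timeline update, while look returns only when it finishes.
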(event EventOnPush
  (params (Player :type BP%20Player%20Object%20Reference))
  ;[1 1 1] Call when the player push the actor
  (Variables|/Script/Engine.CharacterMovementComponent|SetMaxWalkSpeed (Variables|/Script/Engine.Character|GetCharacterMovement Player) (Variables|/Game/Blueprints/Player/BP_Player.BP_Player_C|GetMaxWalkSpeedPushingObject Player)))

(event EventOnDrop
  (params (Player :type BP%20Player%20Object%20Reference))
  ;[1 1 1] Call when the player stop pushing the actor
  (Variables|/Script/Engine.CharacterMovementComponent|SetMaxWalkSpeed (Variables|/Script/Engine.Character|GetCharacterMovement Player) (Variables|/Game/Blueprints/Player/BP_Player.BP_Player_C|GetBaseMaxWalkSpeed Player)))

(event EventOnUseInteract
  (params (Player :type BP%20Player%20Object%20Reference))
  (bind _playerstandingposition (Variables|Default|GetPlayerStandingPosition))
  (bind _returnvalue (Transformation|GetWorldTransform _playerstandingposition))
  (Variables|Default|SetPlayer Player)
  ;[1 1 1] Call when the player is not on the chair
  (Default|UnbindLook (Variables|Default|GetPlayer))
  (Default|UnbindMovement (Variables|Default|GetPlayer))
  (Variables|Default|SetCurrentTransform (Transformation|GetWorldTransform (Variables|/Script/Engine.Character|GetCapsuleComponent (Variables|Default|GetPlayer))))
  (bind _goingonchair (Timeline|Timeline_0 PlayFromStart)
    (:Update
      (Transformation|SetWorldTransform (Variables|/Script/Engine.Character|GetCapsuleComponent (Variables|Default|GetPlayer)) (Math|Transform|Lerp(Transform) (Variables|Default|GetCurrentTransform) (Math|Transform|MakeTransform (.location _returnvalue) (.rotation _returnvalue) "1,1,1") _goingonchair) false false)
      (Default|DefaultMovementBind (Variables|Default|GetPlayer)))
    (:Finished
      (Default|DefaultLookBind (Variables|Default|GetPlayer)))))

(fn ConstructionScript)