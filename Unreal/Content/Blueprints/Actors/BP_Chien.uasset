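; BP_Chien is an interactable dog actor that moves aside when its door component accepts the interacting player's inventory.
; On a successful check, it plays a one-shot standing animation while a timeline interpolates the skeletal mesh's relative position and rotation to a fixed offset.
; When the timeline finishes, the dog loops a sitting animation.
; The locked-open handler always returns false.
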(event EventOnInteract
  (params (Player :type BP%20Player%20Object%20Reference))
  (bind _skeletalmesh (Variables|Default|GetSkeletalMesh))
  (bind _canopen (Default|CanOpen (Variables|Default|GetBP_SC_Door) (Variables|/Game/Blueprints/Player/BP_Player.BP_Player_C|GetInventory Player)))
  (if _canopen
    (Components|Animation|PlayAnimation _skeletalmesh "/Game/Assets/Chien/ChienDebout.ChienDebout" false)
    (bind _newtrack_0 (Timeline|Timeline_0 Play)
      (:Update
        (Transformation|SetRelativeLocationAndRotation (Variables|Default|GetSkeletalMesh) (Math|Vector|Lerp(Vector) "0, 0, 0" "0.000000,100.000000,-30.000000" _newtrack_0) (Math|Rotator|Lerp(Rotator) "0, 0, 0" "0,80.000000, 0" _newtrack_0) false false))
      (:Finished
        (Components|Animation|PlayAnimation _skeletalmesh "/Game/Assets/Chien/ChienAssis_Anim.ChienAssis_Anim" true)))))

(fn ConstructionScript)

(fn OnOpenLocked
  (params (Player :type BP%20Player%20Object%20Reference))
  (return false))