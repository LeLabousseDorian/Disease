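; BP_DigitalClock is an actor that displays the current real-world time as a digital clock.
; Every Tick it reads Now, takes the 12-hour hour and the minute, and writes each to the Hours and Minutes text components.
; The integers are converted directly to text with default formatting, and the construction script is empty.
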(event EventTick
  (params (DeltaSeconds :type Float%20%28single-precision%29))
  (bind _returnvalue (Math|DateTime|Now))
  (bind _output_get (Variables|Default|SetHour (Class|KismetMathLibrary|GetHour12 _returnvalue)))
  (bind _output_get_2 (Variables|Default|SetMinute (Class|KismetMathLibrary|GetMinute _returnvalue)))
  (Rendering|Components|TextRender|SetText (Variables|Default|GetHours) (Utilities|Text|ToText(Integer) _output_get))
  (Rendering|Components|TextRender|SetText (Variables|Default|GetMinutes) (Utilities|Text|ToText(Integer) _output_get_2)))

(fn ConstructionScript)