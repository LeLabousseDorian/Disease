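; BP_MotherBed is a bed actor with a trigger zone that gradually lowers the player's craziness while they are inside it.
; Box overlap events set a PlayerInside flag, identifying the player by the BPI_CrazynessMultiplier interface; any other actor beginning overlap clears the flag.
; While the flag is set, Tick passes a negative, delta-time-scaled amount to the player controller's AddCrazyness.
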(event OnComponentBeginOverlap(Box)
  (params (OverlappedComponent :type Primitive%20Component%20Object%20Reference) (OtherActor :type Actor%20Object%20Reference) (OtherComp :type Primitive%20Component%20Object%20Reference) (OtherBodyIndex :type Integer) (bFromSweep :type Boolean) (SweepResult :type Hit%20Result%20Structure%20%28by%20ref%29))
  (Variables|Default|SetPlayerInside (Utilities|DoesObjectImplementInterface OtherActor "/Game/Blueprints/Interface/BPI_CrazynessMultiplier.BPI_CrazynessMultiplier_C")))

(event OnComponentEndOverlap(Box)
  (params (OverlappedComponent :type Primitive%20Component%20Object%20Reference) (OtherActor :type Actor%20Object%20Reference) (OtherComp :type Primitive%20Component%20Object%20Reference) (OtherBodyIndex :type Integer))
  (if (Utilities|DoesObjectImplementInterface OtherActor "/Game/Blueprints/Interface/BPI_CrazynessMultiplier.BPI_CrazynessMultiplier_C")
    (Variables|Default|SetPlayerInside false)))

(event EventTick
  (params (DeltaSeconds :type Float%20%28single-precision%29))
  (if (Variables|Default|GetPlayerInside)
    (Default|AddCrazyness (CallFunction|GetMyPlayerController) (* DeltaSeconds -0.25))))

(fn ConstructionScript)