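; BP_Mug is a mug actor that the player can pick up and drop.
; OnPickUp turns off physics simulation and collision on its static mesh, and OnDropDown restores both.
; TransformOffset returns a fixed location and rotation offset that keeps the actor's current scale.
; The construction script applies the Material variable to the mesh's first material slot.
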(event EventOnDropDown
  (bind _staticmesh (Variables|Default|GetStaticMesh))
  ;[1 1 1] Call when it's Droped by the player
  (Collision|SetCollisionEnabled _staticmesh "QueryAndPhysics")
  (Physics|SetSimulatePhysics _staticmesh true))

(event EventOnPickUp
  (params (Player :type BP%20Player%20Object%20Reference))
  (bind _staticmesh (Variables|Default|GetStaticMesh))
  ;[1 1 1] Call when it's Picked by the player
  (Physics|SetSimulatePhysics _staticmesh false)
  (Collision|SetCollisionEnabled _staticmesh "NoCollision"))

(fn ConstructionScript
  (Rendering|Material|SetMaterial (Variables|Default|GetStaticMesh) 0 (Variables|Default|GetMaterial)))

(fn TransformOffset
  (return (Math|Transform|MakeTransform "0.000000,10.000000,22.000000" "0,10.000000, 0" (Transformation|GetActorScale3D))))