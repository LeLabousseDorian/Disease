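; Physics prop that the player can pick up and drop, toggling simulation and collision on its mesh.
; Construction applies the chosen mesh and gives the book mesh (Livre) a randomly colored cover through a dynamic material.
; Hits from non-player actors play an impact sound scaled by impulse, throttled briefly, with the sound assigned one second after BeginPlay.
; TransformOffset returns a slightly raised transform at actor scale.
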(event Collision|EventHit
  (params (MyComp :type Primitive%20Component%20Object%20Reference) (Other :type Actor%20Object%20Reference) (OtherComp :type Primitive%20Component%20Object%20Reference) (bSelfMoved :type Boolean) (HitLocation :type Vector :default "0, 0, 0") (HitNormal :type Vector :default "0, 0, 0") (NormalImpulse :type Vector :default "0, 0, 0") (Hit :type Hit%20Result%20Structure%20%28by%20ref%29))
  (if (not (Utilities|DoesObjectImplementInterface Other "/Game/Blueprints/Interface/BPI_Player.BPI_Player_C"))
    (Utilities|FlowControl|DoOnce false :!label _label
      (:Completed
        (Audio|PlaySoundatLocation (Variables|Default|GetSoundPlayed) HitLocation "0, 0, 0" (Math|Float|Clamp(Float) (/ (.z NormalImpulse) 1.5e+05) 0.0 1.0) 1.0 0.0 0 0 0)
        (Utilities|FlowControl|Delay 0.1)
        (goto _label Reset)))))

(event EventBeginPlay
  (Utilities|FlowControl|Delay 1.0)
  (Variables|Default|SetSoundPlayed "/Game/Assets/Props_Deco/HitGroundSound.HitGroundSound"))

(event EventOnDropDown
  (bind _staticmesh (Variables|Default|GetStaticMesh))
  ;[1 1 1] Call when it's Droped by the player
  (Collision|SetCollisionEnabled _staticmesh "QueryAndPhysics")
  (Physics|SetSimulatePhysics _staticmesh true))

(event EventOnPickUp
  (params (Player :type BP%20Player%20Object%20Reference))
  (bind _staticmesh (Variables|Default|GetStaticMesh))
  ;[1 1 1] Call when it's Picked by the player
  (Physics|SetSimulatePhysics _staticmesh false)
  (Collision|SetCollisionEnabled _staticmesh "NoCollision"))

(fn ConstructionScript
  (Components|StaticMesh|SetStaticMesh (Variables|Default|GetStaticMesh) (Variables|Default|GetMesh))
  (if (== (Variables|Default|GetMesh) "/Game/Assets/Props_Deco/livre.livre")
    (bind _returnvalue (Rendering|Material|CreateDynamicMaterialInstance (Variables|Default|GetStaticMesh) 0 "/Game/Assets/Props_Deco/Materiaux/Couverture.Couverture" "None" :!class /Script/Engine.PrimitiveComponent))
    (Rendering|Material|SetVectorParameterValue _returnvalue "Base Color" (Utilities|Struct|MakeLinearColor (Math|Random|RandomFloatinRange 0.0 1.0) (Math|Random|RandomFloatinRange 0.0 1.0) (Math|Random|RandomFloatinRange 0.0 1.0) 1.0) :!class /Script/Engine.MaterialInstanceDynamic)
    (Rendering|Material|SetMaterial (Variables|Default|GetStaticMesh) 0 _returnvalue)))

(fn TransformOffset
  (return (Math|Transform|MakeTransform "0, 0,12.000000" "0, 0, 0" (Transformation|GetActorScale3D))))