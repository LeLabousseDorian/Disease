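; Teddy bear item the player can pick up, hold and use to gradually reduce Crazyness, at the cost of control and vision.
; Using it locks look and movement while a timeline lifts the bear toward the face and tilts the player's view; stopping reverses this.
; Pickup and drop toggle physics and collision, Tick lowers Crazyness while used, and TransformOffset supplies the in-hand offset.
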(event EventOnStopUsing
  (params (Controller :type BP%20My%20Player%20Controller%20Object%20Reference) (Player :type BP%20Player%20Object%20Reference))
  (bind _offsetinplayerhand (Variables|Default|GetOffsetInPlayerHand))
  ;[1 1 1] Call when actor stop being used
  (Variables|Default|SetUsed false)
  (Default|DefaultLookBind (Variables|Default|GetPlayer))
  (Default|DefaultMovementBind (Variables|Default|GetPlayer))
  (Variables|/Game/Blueprints/Player/BP_Player.BP_Player_C|SetStartRotation (Variables|Default|GetPlayer) (Math|Rotator|MakeRotator (.roll (Variables|/Game/Blueprints/Player/BP_Player.BP_Player_C|GetStartRotation (Variables|Default|GetPlayer))) 0.0 (.yaw (Variables|/Game/Blueprints/Player/BP_Player.BP_Player_C|GetStartRotation (Variables|Default|GetPlayer)))))
  ;[1 1 1] Nounours Goes up, in front of the camera and obstruct most of his vision
  (bind _value (Timeline|NounoursCloserToFace Reverse)
    (:Update
      (Transformation|SetActorRelativeLocation (Math|Vector|Lerp(Vector) (.location _offsetinplayerhand) (+ (.location _offsetinplayerhand) "-10.000000,0.000000,8.000000") _value))
      ;[1 1 1] Player look Down/Up when using/stop using this actor
      (Default|RotateonYaw (Variables|Default|GetPlayer) -75.0 _value))))

(event EventTick
  (params (DeltaSeconds :type Float%20%28single-precision%29))
  ;[1 1 1] Reduce Crazyness over time when it's in use
  (if (Variables|Default|GetUsed)
    (Default|AddCrazyness (CallFunction|GetMyPlayerController) (* DeltaSeconds -0.25))))

(event EventOnStartUsing
  (params (Controller :type BP%20My%20Player%20Controller%20Object%20Reference) (Player :type BP%20Player%20Object%20Reference))
  (bind _offsetinplayerhand (Variables|Default|GetOffsetInPlayerHand))
  ;[1 1 1] Call when actor is used
  (Variables|Default|SetUsed true)
  (Default|UnbindLook (Variables|Default|GetPlayer))
  (Default|UnbindMovement (Variables|Default|GetPlayer))
  (Variables|/Game/Blueprints/Player/BP_Player.BP_Player_C|SetStartRotation (Variables|Default|GetPlayer) (Pawn|GetControlRotation (Variables|Default|GetPlayer) :!class /Script/Engine.Pawn))
  ;[1 1 1] Nounours Goes up, in front of the camera and obstruct most of his vision
  (bind _value (Timeline|NounoursCloserToFace PlayFromStart)
    (:Update
      (Transformation|SetActorRelativeLocation (Math|Vector|Lerp(Vector) (.location _offsetinplayerhand) (+ (.location _offsetinplayerhand) "-10.000000,0.000000,8.000000") _value))
      ;[1 1 1] Player look Down/Up when using/stop using this actor
      (Default|RotateonYaw (Variables|Default|GetPlayer) -75.0 _value))))

(event EventOnDropDown
  (bind _player (Variables|Default|GetPlayer))
  (bind _staticmesh_0 (Variables|Default|GetStaticMesh_0))
  ;[1 1 1] Call when it's Droped by the player
  (Variables|Default|SetUsed false)
  (Collision|SetCollisionEnabled _staticmesh_0 "QueryAndPhysics")
  (Physics|SetSimulatePhysics _staticmesh_0 true)
  (Default|DefaultLookBind _player)
  (Default|DefaultMovementBind _player))

(event EventOnPickUp
  (params (Player :type BP%20Player%20Object%20Reference))
  (bind _staticmesh_0 (Variables|Default|GetStaticMesh_0))
  ;[1 1 1] Call when it's Picked by the player
  (Variables|Default|SetPlayer Player)
  (Physics|SetSimulatePhysics _staticmesh_0 false)
  (Collision|SetCollisionEnabled _staticmesh_0 "NoCollision"))

(fn ConstructionScript)

(fn TransformOffset
  (return (Variables|Default|GetOffsetInPlayerHand)))