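; BP_Veilleuse is a night light item that the player can pick up, drop and use, and that slows the rise of craziness nearby.
; Its sphere sends lower or higher multiplier messages through BPI_CrazynessMultiplier on overlap begin and end, whether lit or not.
; It starts at zero intensity; dropping or using turns it on, while pickup or stopping use turns it off, swapping materials.
; Pickup and drop also toggle physics and collision.
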(event OnComponentBeginOverlap(Sphere)
  (params (OverlappedComponent :type Primitive%20Component%20Object%20Reference) (OtherActor :type Actor%20Object%20Reference) (OtherComp :type Primitive%20Component%20Object%20Reference) (OtherBodyIndex :type Integer) (bFromSweep :type Boolean) (SweepResult :type Hit%20Result%20Structure%20%28by%20ref%29))
  ;[1 1 1] Player enter the AoE and his crazyness increases slower
  (if (Utilities|DoesObjectImplementInterface OtherActor "/Game/Blueprints/Interface/BPI_CrazynessMultiplier.BPI_CrazynessMultiplier_C")
    (Class|BPICrazynessMultiplier|OnLowerMulitplier(Message) OtherActor)))

(event OnComponentEndOverlap(Sphere)
  (params (OverlappedComponent :type Primitive%20Component%20Object%20Reference) (OtherActor :type Actor%20Object%20Reference) (OtherComp :type Primitive%20Component%20Object%20Reference) (OtherBodyIndex :type Integer))
  ;[1 1 1] Player leave the AoE and his crazyness increases faster
  (if (Utilities|DoesObjectImplementInterface OtherActor "/Game/Blueprints/Interface/BPI_CrazynessMultiplier.BPI_CrazynessMultiplier_C")
    (Class|BPICrazynessMultiplier|OnHigherMulitplier(Message) OtherActor)))

(event EventOnPickUp
  (params (Player :type BP%20Player%20Object%20Reference))
  (bind _staticmesh1 (Variables|Default|GetStaticMesh1))
  ;[1 1 1] Call when this actor is Picked by the player
  (CallFunction|TurnOff)
  (Physics|SetSimulatePhysics _staticmesh1 false)
  (Collision|SetCollisionEnabled _staticmesh1 "NoCollision"))

(event EventBeginPlay
  ;[1 1 1] Get the base intensity
  (Variables|Default|SetBaseIntensity (Variables|/Script/Engine.LightComponentBase|GetIntensity (Variables|Default|GetPointLight)))
  (Rendering|Components|Light|SetIntensity (Variables|Default|GetPointLight) 0.0))

(event EventOnStartUsing
  (params (Controller :type BP%20My%20Player%20Controller%20Object%20Reference) (Player :type BP%20Player%20Object%20Reference))
  ;[1 1 1] Call when player use the item
  (CallFunction|Turnon))

(event EventOnStopUsing
  (params (Controller :type BP%20My%20Player%20Controller%20Object%20Reference) (Player :type BP%20Player%20Object%20Reference))
  ;[1 1 1] Call when player stop using the item
  (CallFunction|TurnOff))

(event EventOnDropDown
  (bind _staticmesh1 (Variables|Default|GetStaticMesh1))
  ;[1 1 1] Call when this actor is Droped by the player
  (CallFunction|Turnon)
  (Collision|SetCollisionEnabled _staticmesh1 "QueryAndPhysics")
  (Physics|SetSimulatePhysics _staticmesh1 true))

(fn ConstructionScript)

(fn TurnOff
  (Rendering|Components|Light|SetIntensity (Variables|Default|GetPointLight) 0.0)
  (Rendering|Material|SetMaterial (Variables|Default|GetSkeletalMesh1) 0 "/Game/Assets/Veilleuse/MAT_Plastique_transparent_OFF.MAT_Plastique_transparent_OFF"))

(fn Turnon
  (Rendering|Components|Light|SetIntensity (Variables|Default|GetPointLight) (Variables|Default|GetBaseIntensity))
  (Rendering|Material|SetMaterial (Variables|Default|GetSkeletalMesh1) 0 "/Game/Assets/Veilleuse/MAT_Plastique_transparent_ON.MAT_Plastique_transparent_ON"))

(fn TransformOffset
  (return (Math|Transform|MakeTransform "0.000000, 0,15.000000" "0, 0, 0" (Transformation|GetActorScale3D))))