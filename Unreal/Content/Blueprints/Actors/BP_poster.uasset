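; BP_poster is a pickable poster that the player can carry and stick onto a cave door.
; Pick-up and drop toggle its physics and collision, and TransformOffset supplies a relative transform, likely for holding.
; On use, a short forward trace looks for a BPI_CaveDoor actor, sets its poster message, and makes the player drop the poster.
; The poster then attaches at the impact point, aligned to the door, and switches to its unrolled mesh.
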(event EventOnPickUp
  (params (Player :type BP%20Player%20Object%20Reference))
  (bind _poster (Variables|Default|GetPoster))
  (Physics|SetSimulatePhysics _poster false)
  (Collision|SetCollisionEnabled _poster "NoCollision"))

(event EventOnDropDown
  (bind _poster (Variables|Default|GetPoster))
  (Collision|SetCollisionEnabled _poster "QueryAndPhysics")
  (Physics|SetSimulatePhysics _poster true))

(event EventOnStartUsing
  (params (Controller :type BP%20My%20Player%20Controller%20Object%20Reference) (Player :type BP%20Player%20Object%20Reference))
  (bind _poster (Variables|Default|GetPoster))
  (bind _poster_2 (Variables|Default|GetPoster))
  (bind _returnvalue (Transformation|GetWorldLocation _poster_2))
  ;[1 1 1] When used, check if there's an actor that has the Destroyable interface, if it has position the poster at the impact point
  (bind (_outhit _returnvalue_2) (Collision|LineTraceByChannel _returnvalue (+ _returnvalue (* (Math|Vector|GetForwardVector _poster_2) 1e+02) "0,0,-16.000000") "TraceTypeQuery1" false 0 "None"))
  (if _returnvalue_2
    (if (Utilities|DoesObjectImplementInterface (.HitActor (Collision|BreakHitResult _outhit)) "/Game/Blueprints/Interface/BPI_CaveDoor.BPI_CaveDoor_C")
      (Class|BPICaveDoor|SetPoster(Message) (.HitActor (Collision|BreakHitResult _outhit)) true)
      (Default|DropPickableActor Player)
      (Transformation|AttachComponentToComponent (Variables|Default|GetPoster) (.HitComponent (Collision|BreakHitResult _outhit)) "None" "SnapToTarget" "SnapToTarget" "KeepRelative" true)
      (Physics|SetSimulatePhysics _poster false)
      (Collision|SetCollisionEnabled _poster "NoCollision")
      (Transformation|SetWorldLocationAndRotation (Variables|Default|GetPoster) (.ImpactPoint (Collision|BreakHitResult _outhit)) (Math|Rotator|MakeRotator (.roll (Transformation|GetActorRotation (.HitActor (Collision|BreakHitResult _outhit)))) (+ (.pitch (Transformation|GetActorRotation (.HitActor (Collision|BreakHitResult _outhit)))) 9e+01) (.yaw (Transformation|GetActorRotation (.HitActor (Collision|BreakHitResult _outhit))))) false false)
      (Components|StaticMesh|SetStaticMesh (Variables|Default|GetPoster) "/Game/Assets/Affiche/Affiche_unroll.Affiche_unroll"))))

(fn ConstructionScript)

(fn TransformOffset
  (return (Math|Transform|MakeTransform "10.000000,0.000000,15.000000" "0,0.000000, 0" (Transformation|GetActorScale3D))))