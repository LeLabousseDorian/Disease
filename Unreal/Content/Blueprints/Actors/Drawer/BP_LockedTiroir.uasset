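; Locked drawer that slides open or closed when a player carrying the required key interacts with it.
; On BeginPlay it copies the needed key from its parent BP_Drawer actor.
; On interact it searches the player's inventory for that key, and a FlipFlop plays or reverses a timeline that lerps the mesh along local X.
; OnOpenLocked always returns false.
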(event EventOnInteract
  (params (Player :type BP%20Player%20Object%20Reference))
  ;[1 1 1] If the player has the key needed to open this drawer, open it
  (bind _array_element (Utilities|Array|ForEachLoopwithBreak (Variables|/Game/Blueprints/Player/BP_Player.BP_Player_C|GetInventory Player) :!label _label)
    (:LoopBody
      (if (== _array_element (Variables|Default|GetKeyNeeded))
        (Utilities|FlowControl|Sequence
          (:then_0
            (goto _label Break))
          (:then_1
            (Utilities|FlowControl|FlipFlop
              (:A
                (bind _newtrack_0 (Timeline|Timeline_1 Play)
                  (:Update
                    (Transformation|SetRelativeLocation (Variables|Default|GetStaticMesh) (Math|Vector|Lerp(Vector) "0, 0, 0" "40.000000,0.000000, 0" _newtrack_0) false false))))
              (:B
                (Timeline|Timeline_1 Reverse)))))))))

(event EventBeginPlay
  (bind _asbp_drawer (Utilities|Casting|CastToBP_Drawer (Actor|GetParentActor)))
  (Variables|Default|SetKeyNeeded (Variables|/Game/Blueprints/Actors/Drawer/BP_Drawer.BP_Drawer_C|GetKeyNeeded _asbp_drawer)))

(fn ConstructionScript
  (|CallParentFunction))

(fn OnOpenLocked
  (params (Player :type BP%20Player%20Object%20Reference))
  (return false))