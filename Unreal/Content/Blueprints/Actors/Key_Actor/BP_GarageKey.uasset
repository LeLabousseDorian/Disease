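; BP_GarageKey is a lootable garage key actor that the player picks up.
; On loot, it adds its key data from the inventory item component to the player's inventory, triggers a dialogue message and plays a 2D sound.
; It then starts the referenced level sequence and destroys itself, while its construction script only calls the parent's.
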(event EventOnLoot
  (params (Player :type BP%20Player%20Object%20Reference))
  (Utilities|Array|Add (Variables|/Game/Blueprints/Player/BP_Player.BP_Player_C|GetInventory Player) (Variables|/Game/Blueprints/Components/BP_AC_InventoryItem.BP_AC_InventoryItem_C|GetKeyData (Variables|Default|GetBP_AC_InventoryItem)))
  (Class|BPIPlayDialogue|OnPlayDialogue(Message) (Variables|Default|GetBP_SC_Dialogue) Player)
  (Audio|PlaySound2D "/Game/Assets/Key/KeySound.KeySound" 1.0 1.0 0.0 0 0)
  (Sequencer|Player|Play (Variables|/Script/LevelSequence.LevelSequenceActor|GetSequencePlayer (Variables|Default|GetSequence%20toLaunch)) :!class /Script/MovieScene.MovieSceneSequencePlayer)
  (Actor|DestroyActor))

(fn ConstructionScript
  (|CallParentFunction))