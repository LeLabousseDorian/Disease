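; Bottom part of a kitchen drawer that a player can open and close only while carrying the required key.
; On BeginPlay it casts its parent actor to BP_Kitchen_Drawer and copies that drawer's KeyNeeded.
; On interact it searches the player's inventory for that key, then a FlipFlop alternately plays and reverses a timeline.
; The timeline lerps the Drawer component's relative rotation through a quarter turn.
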(event EventOnInteract
  (params (Player :type BP%20Player%20Object%20Reference))
  (bind _array_element (Utilities|Array|ForEachLoopwithBreak (Variables|/Game/Blueprints/Player/BP_Player.BP_Player_C|GetInventory Player) :!label _label)
    (:LoopBody
      (if (== _array_element (Variables|Default|GetKey%20Needed))
        (Utilities|FlowControl|Sequence
          (:then_0
            (goto _label Break))
          (:then_1
            (Utilities|FlowControl|FlipFlop
              (:A
                (bind _open_close (Timeline|Timeline_0 Play)
                  (:Update
                    (Transformation|SetRelativeRotation (Variables|Default|GetDrawer) (Math|Rotator|Lerp(Rotator) "0, 0, 0" "0,-90.000000, 0" _open_close) false false))))
              (:B
                (Timeline|Timeline_0 Reverse)))))))))

(event EventBeginPlay
  (bind _asbp_kitchen_drawer (Utilities|Casting|CastToBP_Kitchen_Drawer (Actor|GetParentActor)))
  (Variables|Default|SetKey%20Needed (Variables|/Game/Blueprints/Actors/Kitchen_Drawer/BP_Kitchen_Drawer.BP_Kitchen_Drawer_C|GetKeyNeeded _asbp_kitchen_drawer)))

(fn ConstructionScript)