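; BP_SC_Dialogue is a dialogue component that shows lines on the player's text widget.
; On OnPlayDialogue, it requires the player's last inventory entry to match SequenceKey and a random roll to pass ProcChance.
; It then sends a timed line to ShowLine, either random or sequential from Dialogues, advancing CurrentDialogue without a bounds check.
; A PlayOnce flag feeds a DoOnce node whose Completed output is empty.
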(event EventOnPlayDialogue
  (params (Player :type BP%20Player%20Object%20Reference))
  (bind _inventory (Variables|/Game/Blueprints/Player/BP_Player.BP_Player_C|GetInventory Player))
  (Variables|Default|SetText%20Widget (Variables|/Game/Blueprints/Player/BP_Player.BP_Player_C|GetTextWidget Player))
  (if (== (Utilities|Array|Get(acopy) _inventory (Utilities|Array|LastIndex _inventory)) (Variables|Default|GetSequenceKey))
    (if (<= (Math|Random|RandomFloat) (Variables|Default|GetProcChance))
      (if (Variables|Default|GetPlayOnce)
        (Utilities|FlowControl|DoOnce false
          (:Completed
            _)))
      (if (Variables|Default|GetRandomText)
        (Default|ShowLine (Variables|Default|GetText%20Widget) (.OutItem (Utilities|Array|Random (Variables|Default|GetDialogues))) (Variables|Default|GetTime%20Active))
        (else
          (Default|ShowLine (Variables|Default|GetText%20Widget) (Utilities|Array|Get(acopy) (Variables|Default|GetDialogues) (Variables|Default|GetCurrentDialogue)) (Variables|Default|GetTime%20Active))
          (Variables|Default|SetCurrentDialogue (+ (Variables|Default|GetCurrentDialogue) 1)))))))