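; AI controller for the Father character, which periodically sends him to a random room.
; Init sets up the BB_Father blackboard, stores the player character in it and runs BT_Father.
; A Delay on Tick acts as a repeating timer that flags ChangingRoom and writes a random RoomsLocation entry to RandomRoomLoc.
; The random index is bounded exclusively by LastIndex, so the final room is never picked.
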(event Custom|Init
  (bind _blackboardcomponent (Class|AIController|UseBlackboard "/Game/Blueprints/Father/BB_Father.BB_Father"))
  (bind _output_get (Variables|Default|SetBlackboard%20Component _blackboardcomponent))
  (AI|Components|Blackboard|SetValueasObject _output_get (Utilities|Name|MakeLiteralName "Player") (Game|GetPlayerCharacter 0))
  (AI|RunBehaviorTree "/Game/Blueprints/Father/BT_Father.BT_Father"))

(event EventTick
  (params (DeltaSeconds :type Float%20%28single-precision%29))
  (Utilities|FlowControl|Delay 3e+01)
  (bind _blackboard_component (Variables|Default|GetBlackboard%20Component)
    (:then
      (AI|Components|Blackboard|SetValueasBool _blackboard_component (Utilities|Name|MakeLiteralName "ChangingRoom") true)
      (AI|Components|Blackboard|SetValueasVector (Variables|Default|GetBlackboard%20Component) (Utilities|Name|MakeLiteralName "RandomRoomLoc") (Utilities|Array|Get(acopy) (Variables|Default|GetRoomsLocation) (Math|Random|RandomInteger (Utilities|Array|LastIndex (Variables|Default|GetRoomsLocation))))))
    (:else)))

(fn ConstructionScript)