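; BP_Father is an AI enemy that spots and kills the player.
; Pawn sensing sets a CanSee blackboard key, which a retriggerable delay clears shortly after the last sighting.
; Player overlap makes the player drop held objects, lose controls and receive a death message while a kill animation plays.
; A second collision destroys cave doors with posters attached, and StopMoving and StartMoving events toggle walk speed.
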(event OnSeePawn(PawnSensing)
  (params (Pawn :type Pawn%20Object%20Reference))
  ;[1 1 1] When player is seen
  (AI|Components|Blackboard|SetValueasBool (Variables|Default|GetMyBlackboard) (Utilities|Name|MakeLiteralName "CanSee") true)
  (Utilities|FlowControl|RetriggerableDelay 0.6)
  (AI|Components|Blackboard|SetValueasBool (Variables|Default|GetMyBlackboard) (Utilities|Name|MakeLiteralName "CanSee") false))

(event OnComponentBeginOverlap(CollisionWithCaveDoor)
  (params (OverlappedComponent :type Primitive%20Component%20Object%20Reference) (OtherActor :type Actor%20Object%20Reference) (OtherComp :type Primitive%20Component%20Object%20Reference) (OtherBodyIndex :type Integer) (bFromSweep :type Boolean) (SweepResult :type Hit%20Result%20Structure%20%28by%20ref%29))
  ;[1 1 1] When a door with a poster enter the collision, destroy it
  (Variables|Default|SetHitActor OtherActor)
  (bind _hasposter (Class|BPICaveDoor|HasPosterAttached(Message) (Variables|Default|GetHitActor)))
  (if (and _hasposter (Utilities|DoesObjectImplementInterface (Variables|Default|GetHitActor) "/Game/Blueprints/Interface/BPI_CaveDoor.BPI_CaveDoor_C"))
    (Class|BPICaveDoor|Destroy(Message) (Variables|Default|GetHitActor))))

(event OnComponentBeginOverlap(CollisionWithPlayer)
  (params (OverlappedComponent :type Primitive%20Component%20Object%20Reference) (OtherActor :type Actor%20Object%20Reference) (OtherComp :type Primitive%20Component%20Object%20Reference) (OtherBodyIndex :type Integer) (bFromSweep :type Boolean) (SweepResult :type Hit%20Result%20Structure%20%28by%20ref%29))
  (bind _mesh (Variables|Character|GetMesh))
  ;[1 1 1] Kill Player when he enter the collision
  (if (Utilities|DoesObjectImplementInterface (Variables|Default|GetHitActor) "/Game/Blueprints/Interface/BPI_Player.BPI_Player_C")
    (Variables|Default|SetHitActor OtherActor)
    (bind _asbp_player (Utilities|Casting|CastToBP_Player (Variables|Default|GetHitActor)))
    (Default|DropPickableActor _asbp_player)
    (Default|DropPushActor _asbp_player)
    (Default|UnbindMovement _asbp_player)
    (Default|UnbindLook _asbp_player)
    (Components|Animation|PlayAnimation _mesh "/Game/Blueprints/Father/FatherAnim/death.death" false)
    (Class|BPIPlayer|OnDeath(Message) _asbp_player self)
    (Utilities|FlowControl|Delay 0.9)
    (Components|Animation|SetAnimationMode _mesh "AnimationBlueprint")))

(event Custom|StopMoving
  (Variables|/Script/Engine.CharacterMovementComponent|SetMaxWalkSpeed (Variables|Character|GetCharacterMovement) 0.0))

(event Custom|StartMoving
  (Variables|/Script/Engine.CharacterMovementComponent|SetMaxWalkSpeed (Variables|Character|GetCharacterMovement) (Variables|Default|GetDefaultWalkSpeed)))

(event EventBeginPlay
  (bind _output_get (Variables|Default|SetMyBlackboard (AI|GetBlackboard (Pawn|GetController))))
  (AI|Components|Blackboard|SetValueasBool _output_get (Utilities|Name|MakeLiteralName "CanSee") false)
  (Variables|Default|SetDefaultWalkSpeed (Variables|/Script/Engine.CharacterMovementComponent|GetMaxWalkSpeed (Variables|Character|GetCharacterMovement))))

(fn ConstructionScript)