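; Player controller that relays input to dispatch calls and manages the player's "crazyness" level.
; Movement, look, interact, item, crazyness-reduction and Start inputs are forwarded, with Start alternating pressed and released calls via FlipFlop.
; A delayed Tick adds delta time scaled by a multiplier to crazyness, clamped and broadcast for post-process updates.
; It caches the controlled BP_Player on BeginPlay, and MyPosses blends the view to that character.
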(event Custom|PostProcessTick
  (params (Value :type Float%20%28single-precision%29))
  ;[1 1 1] Add crazy value over time
  (CallFunction|AddCrazyness (* Value (Variables|Character|GetAddedCrazynessOverTimeMultiplier))))

(event Custom|MyPosses
  (Game|Player|SetViewTargetwithBlend (Variables|Character|GetMyCharacter) 1.0 "VTBlend_Linear" 0.0 false))

(event EventBeginPlay
  ;[1 0 0] Get the Player (need to change to an event system)
  (|GetPlayerRef))

(event EventTick
  (params (DeltaSeconds :type Float%20%28single-precision%29))
  (Utilities|FlowControl|Delay 0.1)
  (CallFunction|PostProcessTick DeltaSeconds))

(event Input|ActionEvents|InputActionInteract
  (params (Key :type Key%20Structure :default "None"))
  ;[1 1 1] Interact
  (:Pressed
    (Default|CallOnInteractPressed))
  (:Released
    (Default|CallOnInteractReleased)))

(event Input|ActionEvents|InputActionUseItem
  (params (Key :type Key%20Structure :default "None"))
  ;[1 1 1] Use Item
  (:Pressed
    (Default|CallOnUseItemPressed))
  (:Released
    (Default|CallOnUseItemReleased)))

(event Input|ActionEvents|InputActionStart
  (params (Key :type Key%20Structure :default "None"))
  ;[1 1 1] Start
  (:Pressed
    (Utilities|FlowControl|FlipFlop
      (:A
        (Default|CallOnStartPressed))
      (:B
        (Default|CallOnStartReleased)))))

(event Input|ActionEvents|InputActionDropItem
  (params (Key :type Key%20Structure :default "None"))
  ;[1 1 1] Drop item
  (:Pressed
    (Default|CallOnDropItemPressed)))

(event Input|AxisEvents|InputAxisReduceCrazyness
  (params (AxisValue :type Float%20%28single-precision%29))
  ;[1 1 1] Use Item
  (Default|CallOnReduceCrazyness AxisValue))

(event Input|AxisEvents|InputAxisTurn
  (params (AxisValue :type Float%20%28single-precision%29))
  ;[1 1 1] Mouse Axis
  (Default|CallOnLookRight AxisValue))

(event Input|AxisEvents|InputAxisLookUp
  (params (AxisValue :type Float%20%28single-precision%29))
  ;[1 1 1] Mouse Axis
  (Default|CallOnLookUp AxisValue))

(event Input|AxisEvents|InputAxisMoveForward
  (params (AxisValue :type Float%20%28single-precision%29))
  ;[1 1 1] KeyboardMovement + Left Stick
  (Default|CallOnMoveForward AxisValue))

(event Input|AxisEvents|InputAxisMoveRight
  (params (AxisValue :type Float%20%28single-precision%29))
  ;[1 1 1] KeyboardMovement + Left Stick
  (Default|CallOnMoveRight AxisValue))

(event Input|AxisEvents|InputAxisTurnRate
  (params (AxisValue :type Float%20%28single-precision%29))
  ;[1 1 1] Right Stick
  (Default|CallOnLookRight AxisValue))

(event Input|AxisEvents|InputAxisLookUpRate
  (params (AxisValue :type Float%20%28single-precision%29))
  ;[1 1 1] Right Stick
  (Default|CallOnLookUp AxisValue))

(fn ConstructionScript)

(fn AddCrazyness
  (params (Value :type Float%20%28single-precision%29))
  (bind _output_get (Variables|Character|SetCrazyness (Math|Float|Clamp(Float) (+ Value (Variables|Character|GetCrazyness)) 0.0 3.0)))
  (Default|CallOnUpdatePostProcess _output_get))

(fn UpdatePostProcess
  (Default|UpdatePostProcess (Variables|Character|GetMyCharacter) 0.0))

(fn SetTurnYAxisMultiplier
  (params (TurnYAxisMultiplier :type Float%20%28single-precision%29))
  (Variables|Character|SetTurnYAxisMultiplier TurnYAxisMultiplier))