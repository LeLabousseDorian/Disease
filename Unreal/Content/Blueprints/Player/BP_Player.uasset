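; First-person player character that looks, moves, picks up, pushes, loots and uses actors through interfaces.
; Default bind functions subscribe to player controller dispatchers, and holding or pushing an item rebinds those inputs to change their actions.
; Camera line traces drive interactions, while a raycasting component toggles the hand widget.
; It also handles the pause menu, craziness-driven post-process and multiplier changes, and a timed death-and-respawn teleport.
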(event OnRaycastHit(BP_AC_MyRaycasting)
  (params (ActorHitted :type Actor%20Object%20Reference))
  (bind _handwidget (Variables|Default|GetHandWidget))
  ;[1 1 1] Show Hand UI when hovering Interactable Actor
  (if (Utilities|DoesObjectImplementInterface ActorHitted "/Game/Blueprints/Interface/BPI_Interactable.BPI_Interactable_C")
    (if (not (Widget|IsVisible _handwidget))
      (UserInterface|Viewport|AddtoViewport _handwidget 0))
    (else
      (CallFunction|RemoveHUDatBadRaycast))))

(event OnRaycastEnd(BP_AC_MyRaycasting)
  ;[1 1 1] Remove Hand UI
  (CallFunction|RemoveHUDatBadRaycast))

(event Custom|RemoveHUDAtBadRaycast
  ;[1 1 1] Remove Hand UI
  (Widget|RemovefromParent (Variables|Default|GetHandWidget)))

(event EventBeginPlay
  (Utilities|FlowControl|Sequence
    (:then_0
      ;[1 1 1] Pause Menu Widget
      (bind _returnvalue (UserInterface|CreateWidget "/Game/UI/WBP_PauseMenu.WBP_PauseMenu_C"))
      (Variables|Default|SetPauseMenu _returnvalue)
      (bind _returnvalue_2 (UserInterface|CreateWidget "/Game/UI/WBP_Grab.WBP_Grab_C"))
      (Variables|Default|SetHandWidget _returnvalue_2))
    (:then_1
      ;[1 1 1] Default Bind for the player
      (Binds|DefaultLookBind)
      (Binds|DefaultMovementBind)
      (Binds|DefaultInteractBind)
      (Binds|DefaultPauseMenuBind)
      (Binds|DefaultUpdatePostProcessBind)
      (Binds|DefaultUseItemBind)
      (Binds|DefaultUseInteractableBind))
    (:then_2
      (Variables|/Game/Blueprints/Components/BP_AC_MyRaycasting.BP_AC_MyRaycasting_C|SetRaycastOrigin (Variables|Default|GetBP_AC_MyRaycasting) (Variables|MyCharacter|GetFirstPersonCamera)))))

(event EventOnLowerMulitplier
  (bind _myplayercontroller (CallFunction|GetMyPlayerController))
  ;[1 1 1] When entering the Veilleuse AoE the crazyness multiplier
  (Variables|/Game/Blueprints/Player/BP_MyPlayerController.BP_MyPlayerController_C|SetAddedCrazynessOverTimeMultiplier _myplayercontroller (* (Variables|/Game/Blueprints/Player/BP_MyPlayerController.BP_MyPlayerController_C|GetAddedCrazynessOverTimeMultiplier _myplayercontroller) 0.5)))

(event EventOnHigherMulitplier
  (bind _myplayercontroller (CallFunction|GetMyPlayerController))
  ;[1 1 1] When leaving the Veilleuse AoE the crazyness multiplier
  (Variables|/Game/Blueprints/Player/BP_MyPlayerController.BP_MyPlayerController_C|SetAddedCrazynessOverTimeMultiplier _myplayercontroller (* (Variables|/Game/Blueprints/Player/BP_MyPlayerController.BP_MyPlayerController_C|GetAddedCrazynessOverTimeMultiplier _myplayercontroller) 2.0)))

(event EventOnDeath
  ;[1 1 1] Trigger when the player enter the father collision
  (Transformation|Teleport self (Variables|Default|GetDeathLocation) "0, 0, 0")
  (Utilities|FlowControl|Delay 5.0)
  (Transformation|Teleport self (Variables|Default|GetSpawnLocation) "0, 0, 0"))

(fn ConstructionScript)

(fn UpdatePostProcess
  (params (Crazyness :type Float%20%28single-precision%29))
  (Variables|/Script/Engine.CameraComponent|SetPostProcessSettings (Variables|MyCharacter|GetFirstPersonCamera) (Utilities|Struct|MakePostProcessSettings Crazyness)))

(fn LookRight
  (params (AxisValue :type Float%20%28single-precision%29))
  (Pawn|Input|AddControllerYawInput (* AxisValue (Variables|Default|GetBaseTurnRate) (Utilities|Time|GetWorldDeltaSeconds))))

(fn LookUp
  (params (AxisValue :type Float%20%28single-precision%29))
  (Pawn|Input|AddControllerPitchInput (* AxisValue (Variables|Default|GetBaseLookUpRate) (Utilities|Time|GetWorldDeltaSeconds) (Variables|/Game/Blueprints/Player/BP_MyPlayerController.BP_MyPlayerController_C|GetTurnYAxisMultiplier (CallFunction|GetMyPlayerController)))))

(fn DefaultLookBind
  (bind _myplayercontroller (CallFunction|GetMyPlayerController))
  (EventDispatchers|UnbindallEventsfromOnLookRight _myplayercontroller)
  (EventDispatchers|UnbindallEventsfromOnLookUp _myplayercontroller)
  (EventDispatchers|BindEventtoOnLookRight _myplayercontroller (EventDispatchers|CreateEvent :!event LookRight))
  (EventDispatchers|BindEventtoOnLookUp _myplayercontroller (EventDispatchers|CreateEvent :!event LookUp)))

(fn UnbindLook
  (bind _myplayercontroller (CallFunction|GetMyPlayerController))
  (EventDispatchers|UnbindallEventsfromOnLookRight _myplayercontroller)
  (EventDispatchers|UnbindallEventsfromOnLookUp _myplayercontroller))

(fn MoveForward
  (params (AxisValue :type Float%20%28single-precision%29))
  (Pawn|Input|AddMovementInput (Math|Vector|GetForwardVector (Variables|MyCharacter|GetFirstPersonCamera)) AxisValue false))

(fn MoveRight
  (params (AxisValue :type Float%20%28single-precision%29))
  (Pawn|Input|AddMovementInput (Math|Vector|GetRightVector (Variables|MyCharacter|GetFirstPersonCamera)) AxisValue false))

(fn DefaultMovementBind
  (bind _myplayercontroller (CallFunction|GetMyPlayerController))
  (EventDispatchers|UnbindallEventsfromOnMoveForward _myplayercontroller)
  (EventDispatchers|UnbindallEventsfromOnMoveRight _myplayercontroller)
  (EventDispatchers|BindEventtoOnMoveForward _myplayercontroller (EventDispatchers|CreateEvent :!event MoveForward))
  (EventDispatchers|BindEventtoOnMoveRight _myplayercontroller (EventDispatchers|CreateEvent :!event MoveRight)))

(fn DefaultInteract
  ;[1 1 1] Interact Input (no item) check what interface the actor implement
  (bind (_outhit _returnvalue) (CallFunction|CustomRaycast))
  (if _returnvalue
    (Utilities|FlowControl|Sequence
      (:then_0
        (Action|HitPickable _outhit)
        (Action|HitKey _outhit)
        (Action|HitInteract _outhit)
        (Action|HitPushObject _outhit)))))

(fn IteminHandInteract
  ;[1 1 1] Interact Input (with item)
  (bind (_outhit _returnvalue) (CallFunction|CustomRaycast))
  (if _returnvalue
    (Action|HitInteract _outhit)
    (Action|HitKey _outhit)))

(fn HitPickable
  (params (Hit :type Hit%20Result%20Structure%20%28by%20ref%29))
  (bind _hitactor (Collision|BreakHitResult Hit))
  ;[1 1 1] If the actor hit implement the ActorPickable interface, then Attach it to the player
  (if (Utilities|DoesObjectImplementInterface _hitactor "/Game/Blueprints/Interface/BPI_ActorPickable.BPI_ActorPickable_C")
    (Class|BPIActorPickable|OnPickUp(Message) _hitactor self)
    (bind _output_get (Variables|ObjectHeld|SetActorHeld _hitactor))
    (Transformation|AttachComponentToComponent _output_get (Variables|Default|GetObjectHeld) "None" "SnapToTarget" "SnapToTarget" "KeepRelative" true)
    ;;[1 0 0] Placer l'offset dans l'acteur pas dans le player
    (bind _offset (Class|BPIActorPickable|TransformOffset(Message) (Variables|ObjectHeld|GetActorHeld)))
    (Class|SceneComponent|AddLocalTransform (Variables|/Script/Engine.Actor|GetRootComponent (Variables|ObjectHeld|GetActorHeld)) _offset false false)
    (Binds|PickableActorHeldBind)))

(fn HitInteract
  (params (Hit :type Hit%20Result%20Structure%20%28by%20ref%29))
  (bind _hitactor (Collision|BreakHitResult Hit))
  ;[1 1 1] On interactable hit
  (if (Utilities|DoesObjectImplementInterface _hitactor "/Game/Blueprints/Interface/BPI_Interactable.BPI_Interactable_C")
    (Class|BPIInteractable|OnInteract(Message) _hitactor self)))

(fn HitUsableInteract
  (params (Hit :type Hit%20Result%20Structure%20%28by%20ref%29))
  (bind _hitactor (Collision|BreakHitResult Hit))
  ;[1 1 1] If the actor implement the "Pushable Actor" Interface, then attach it to the player
  (if (Utilities|DoesObjectImplementInterface _hitactor "/Game/Blueprints/Interface/BPI_Interactable.BPI_Interactable_C")
    (Class|BPIInteractable|OnUseInteract(Message) _hitactor self)))

(fn HitPushObject
  (params (Hit :type Hit%20Result%20Structure%20%28by%20ref%29))
  (bind _hitactor (Collision|BreakHitResult Hit))
  ;[1 1 1] If the actor implement the "Pushable Actor" Interface, then attach it to the player
  (if (Utilities|DoesObjectImplementInterface _hitactor "/Game/Blueprints/Interface/BPI_PushableActor.BPI_PushableActor_C")
    (Class|BPIPushableActor|OnPush(Message) _hitactor self)
    (bind _output_get (Variables|ObjectHeld|SetActorHeld _hitactor))
    (Transformation|AttachComponentToComponent _output_get (Variables|Default|GetObjectPush) "None" "KeepWorld" "KeepWorld" "KeepWorld" true)
    (Binds|PushActorHeldBind)))

(fn HitKey
  (params (Hit :type Hit%20Result%20Structure%20%28by%20ref%29))
  (bind _hitactor (Collision|BreakHitResult Hit))
  ;[1 1 1] If the actor hit implement the "Lootable" Interface
  (if (Utilities|DoesObjectImplementInterface _hitactor "/Game/Blueprints/Interface/BPI_Lootable.BPI_Lootable_C")
    (Class|BPILootable|OnLoot(Message) _hitactor self)))

(fn UnbindMovement
  (bind _myplayercontroller (CallFunction|GetMyPlayerController))
  (EventDispatchers|UnbindallEventsfromOnMoveForward _myplayercontroller)
  (EventDispatchers|UnbindallEventsfromOnMoveRight _myplayercontroller))

(fn DefaultInteractBind
  (bind _myplayercontroller (CallFunction|GetMyPlayerController))
  (EventDispatchers|UnbindallEventsfromOnInteractPressed _myplayercontroller)
  (EventDispatchers|UnbindallEventsfromOnInteractReleased _myplayercontroller)
  (EventDispatchers|UnbindallEventsfromOnDropItemPressed _myplayercontroller)
  (EventDispatchers|BindEventtoOnInteractPressed _myplayercontroller (EventDispatchers|CreateEvent :!event DefaultInteract)))

(fn DefaultPauseMenuBind
  (bind _myplayercontroller (CallFunction|GetMyPlayerController))
  (EventDispatchers|UnbindallEventsfromOnStartPressed _myplayercontroller)
  (EventDispatchers|UnbindallEventsfromOnStartReleased _myplayercontroller)
  (EventDispatchers|BindEventtoOnStartPressed _myplayercontroller (EventDispatchers|CreateEvent :!event ShowPauseMenu))
  (EventDispatchers|BindEventtoOnStartReleased _myplayercontroller (EventDispatchers|CreateEvent :!event HidePauseMenu)))

(fn DefaultUpdatePostProcessBind
  (bind _myplayercontroller (CallFunction|GetMyPlayerController))
  (EventDispatchers|UnbindallEventsfromOnUpdatePostProcess _myplayercontroller)
  (EventDispatchers|BindEventtoOnUpdatePostProcess _myplayercontroller (EventDispatchers|CreateEvent :!event UpdatePostProcess)))

(fn DefaultUseItemBind
  (bind _myplayercontroller (CallFunction|GetMyPlayerController))
  (EventDispatchers|UnbindallEventsfromOnUseItemPressed _myplayercontroller)
  (EventDispatchers|UnbindallEventsfromOnUseItemReleased _myplayercontroller)
  (EventDispatchers|BindEventtoOnUseItemPressed _myplayercontroller (EventDispatchers|CreateEvent :!event UseItem))
  (EventDispatchers|BindEventtoOnUseItemReleased _myplayercontroller (EventDispatchers|CreateEvent :!event StopUsingItem)))

(fn DefaultUseInteractableBind
  (bind _myplayercontroller (CallFunction|GetMyPlayerController))
  (EventDispatchers|UnbindallEventsfromOnUseInteractablePressed _myplayercontroller)
  (EventDispatchers|UnbindallEventsfromOnUseInteractableReleased _myplayercontroller)
  (EventDispatchers|BindEventtoOnUseInteractablePressed _myplayercontroller (EventDispatchers|CreateEvent :!event DefaultUseInteractable)))

(fn PickableActorHeldBind
  (bind _myplayercontroller (CallFunction|GetMyPlayerController))
  (EventDispatchers|UnbindallEventsfromOnInteractPressed _myplayercontroller)
  (EventDispatchers|UnbindallEventsfromOnDropItemPressed _myplayercontroller)
  (EventDispatchers|BindEventtoOnInteractPressed _myplayercontroller (EventDispatchers|CreateEvent :!event IteminHandInteract))
  (EventDispatchers|BindEventtoOnDropItemPressed _myplayercontroller (EventDispatchers|CreateEvent :!event DropPickableActor)))

(fn DropPickableActor
  ;[1 1 1] Player drop the actor he's holding (call "on stop using" before dropping the item to avoid bug)
  ;;[1 0 0] Placer l'offset dans l'acteur pas dans le player
  (Transformation|AddActorWorldOffset (Variables|ObjectHeld|GetActorHeld) (* (Transformation|GetActorForwardVector) 5e+01))
  (Transformation|SetActorRotation (Variables|ObjectHeld|GetActorHeld) (Math|Rotator|MakeRotator 0.0 0.0 (.yaw (Transformation|GetActorRotation (Variables|ObjectHeld|GetActorHeld)))))
  (Transformation|DetachFromActor (Variables|ObjectHeld|GetActorHeld) "KeepWorld" "KeepWorld" "KeepWorld")
  (Class|BPIActorPickable|OnDropDown(Message) (Variables|ObjectHeld|GetActorHeld))
  (Variables|ObjectHeld|SetActorHeld 0)
  (Binds|DefaultInteractBind))

(fn DropPushActor
  ;[1 1 1] Player is pushing an item
  (Transformation|DetachFromActor (Variables|ObjectHeld|GetActorHeld) "KeepWorld" "KeepWorld" "KeepWorld")
  (Class|BPIPushableActor|OnDrop(Message) (Variables|ObjectHeld|GetActorHeld) self)
  (Variables|ObjectHeld|SetActorHeld 0)
  (Binds|DefaultInteractBind)
  (Binds|DefaultUseInteractableBind))

(fn PushActorHeldBind
  (bind _myplayercontroller (CallFunction|GetMyPlayerController))
  (EventDispatchers|UnbindallEventsfromOnInteractPressed _myplayercontroller)
  (EventDispatchers|UnbindallEventsfromOnDropItemPressed _myplayercontroller)
  (EventDispatchers|UnbindallEventsfromOnUseInteractablePressed _myplayercontroller)
  (EventDispatchers|BindEventtoOnInteractPressed _myplayercontroller (EventDispatchers|CreateEvent :!event DefaultUseItemBind))
  (EventDispatchers|BindEventtoOnDropItemPressed _myplayercontroller (EventDispatchers|CreateEvent :!event DropPushActor)))

(fn ShowPauseMenu
  (UserInterface|Viewport|AddtoViewport (Variables|Default|GetPauseMenu) 0)
  (Game|SetGamePaused true)
  (Variables|/Script/Engine.PlayerController|SetbShowMouseCursor (Game|GetPlayerController 0) true))

(fn HidePauseMenu
  (Default|ClosePauseMenu (Variables|Default|GetPauseMenu)))

(fn CustomRaycast
  (bind _firstpersoncamera (Variables|MyCharacter|GetFirstPersonCamera))
  (bind _returnvalue (Transformation|GetWorldLocation _firstpersoncamera))
  (bind (_outhit _returnvalue_2) (Collision|LineTraceByChannel _returnvalue (+ _returnvalue (* (Math|Vector|GetForwardVector _firstpersoncamera) (Variables|Default|GetRayCastDistance)) "0,0,-16.000000") "TraceTypeQuery1" false 0 "None" true "(R=1.000000,G=0.000000,B=0.000000,A=1.000000)" "(R=0.000000,G=1.000000,B=0.000000,A=1.000000)" 2.0))
  (return _outhit _returnvalue_2))

(fn UseItem
  (bind _actorheld (Variables|ObjectHeld|GetActorHeld))
  ;[1 1 1] Use the interface "ItemUsable" of the item held
  (if (Utilities|DoesObjectImplementInterface _actorheld "/Game/Blueprints/Interface/BPI_ItemUsable.BPI_ItemUsable_C")
    (Class|BPIItemUsable|OnStartUsing(Message) _actorheld (CallFunction|GetMyPlayerController) self)))

(fn StopUsingItem
  (bind _actorheld (Variables|ObjectHeld|GetActorHeld))
  ;[1 1 1] Use the interface "ItemUsable" of the item held
  (if (Utilities|DoesObjectImplementInterface _actorheld "/Game/Blueprints/Interface/BPI_ItemUsable.BPI_ItemUsable_C")
    (Class|BPIItemUsable|OnStopUsing(Message) _actorheld (CallFunction|GetMyPlayerController) self)))

(fn DefaultUseInteractable
  ;[1 1 1] Raycast to check if there's a Interactable actor in front of the player
  (bind _outhit (CallFunction|CustomRaycast))
  (Action|HitUseInteractable _outhit))

(fn HitUseInteractable
  (params (Hit :type Hit%20Result%20Structure))
  (bind _hitactor (Collision|BreakHitResult Hit))
  ;[1 1 1] Use the interact interface of the actor hit
  (if (Utilities|DoesObjectImplementInterface _hitactor "/Game/Blueprints/Interface/BPI_Interactable.BPI_Interactable_C")
    (Class|BPIInteractable|OnUseInteract(Message) _hitactor self)))

(fn RotateonYaw
  (params (Rotation :type Float%20%28single-precision%29) (Time :type Float%20%28single-precision%29))
  (bind _returnvalue (Pawn|GetControlRotation :!class /Script/Engine.Pawn))
  (Pawn|SetControlRotation (CallFunction|GetMyPlayerController) (Math|Rotator|Lerp(Rotator) (Variables|Default|GetStartRotation) (Math|Rotator|MakeRotator (.roll _returnvalue) Rotation (.yaw _returnvalue)) Time true)))