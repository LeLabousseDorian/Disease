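; BP_Father is an AI enemy that detects pawns by sight and kills the player on contact.
; PawnSensing sets the blackboard CanSee key, and a short retriggerable delay clears it once sightings stop, exposing visibility to the AI logic.
; Overlapping the Collision component sends a death message to any actor implementing BPI_Player.
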(event OnSeePawn(PawnSensing)
  (params (Pawn :type Pawn%20Object%20Reference))
  (AI|Components|Blackboard|SetValueasBool (Variables|Default|GetMyBlackboard) (Utilities|Name|MakeLiteralName "CanSee") true)
  (Utilities|FlowControl|RetriggerableDelay 0.6)
  (AI|Components|Blackboard|SetValueasBool (Variables|Default|GetMyBlackboard) (Utilities|Name|MakeLiteralName "CanSee") false))

(event OnComponentBeginOverlap(Collision)
  (params (OverlappedComponent :type Primitive%20Component%20Object%20Reference) (OtherActor :type Actor%20Object%20Reference) (OtherComp :type Primitive%20Component%20Object%20Reference) (OtherBodyIndex :type Integer) (bFromSweep :type Boolean) (SweepResult :type Hit%20Result%20Structure%20%28by%20ref%29))
  (if (Utilities|DoesObjectImplementInterface OtherActor "/Game/Blueprints/Interface/BPI_Player.BPI_Player_C")
    (Class|BPIPlayer|OnDeath(Message) OtherActor)))

(event EventBeginPlay
  (bind _output_get (Variables|Default|SetMyBlackboard (AI|GetBlackboard (Pawn|GetController))))
  (AI|Components|Blackboard|SetValueasBool _output_get (Utilities|Name|MakeLiteralName "CanSee") false))

(fn ConstructionScript)