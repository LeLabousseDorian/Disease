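; BP_KeyBedroom is a lootable key pickup actor, named for a bedroom.
; Its construction script sets the static mesh from the key data on its BPACInventoryItem component.
; The OnLoot event adds that key data to the looting player's inventory and destroys the actor.
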(event EventOnLoot
  (params (Player :type BP%20Player%20Object%20Reference))
  (Utilities|Array|Add (Variables|/Game/MyFolders/Blueprints/Player/BP_Player.BP_Player_C|GetInventory Player) (Variables|/Game/MyFolders/Blueprints/Components/BP_SC_InventoryItem.BP_AC_InventoryItem_C|GetKeyData (Variables|Default|GetBP_AC_InventoryItem)))
  (Actor|DestroyActor))

(fn ConstructionScript
  (Components|StaticMesh|SetStaticMesh (Variables|Default|GetStaticMesh) (Variables|/Game/MyFolders/Blueprints/DataAsset/BP_DA_KeyParent.BP_DA_KeyParent_C|GetStaticMesh (Variables|/Game/MyFolders/Blueprints/Components/BP_SC_InventoryItem.BP_AC_InventoryItem_C|GetKeyData (Variables|Default|GetBP_AC_InventoryItem)))))