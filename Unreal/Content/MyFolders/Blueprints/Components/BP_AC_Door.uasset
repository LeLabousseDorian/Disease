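; Door component that attaches to a skeletal mesh and checks whether a player's inventory holds the key needed to open it.
; On BeginPlay it caches the parent skeletal mesh and sets its play rate to reverse.
; OpenDoor passes the inventory to CanOpen, which searches for KeyNeededToOpen.
; The result is not yet used, so no opening animation is triggered here.
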(event Custom|OpenDoor
  (params (PlayerInventory :type Array%20of%20BP%20DA%20Key%20Parent%20Object%20References))
  ;[1 1 1] Check if the player has the corresponding key to use animation
  (CallFunction|CanOpen PlayerInventory))

(event EventBeginPlay
  (bind _asskeletal_mesh_component (Utilities|Casting|CastToSkeletalMeshComponent (Transformation|GetAttachParent)))
  (bind _output_get (Variables|Default|SetMySkeletalMesh _asskeletal_mesh_component))
  (Components|Timeline|SetPlayRate _output_get -1.0))

(fn CanOpen
  (params (Array :type Array%20of%20BP%20DA%20Key%20Parent%20Object%20References))
  (for _array_element Array
    (if (== _array_element (Variables|Default|GetKeyNeededToOpen))
      (return true))))