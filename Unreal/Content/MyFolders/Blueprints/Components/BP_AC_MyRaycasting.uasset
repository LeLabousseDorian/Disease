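; Actor component that casts a ray forward from an origin component and reports what it hits through callbacks.
; Each tick it line-traces on the Visibility channel over a set distance, with a slight downward offset at the end point and an actor ignore list.
; A hit passes the actor to OnRaycastHit and sets WasHit.
; WasHit is never cleared here, so OnRaycastEnd repeats on every later miss.
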(event EventTick
  (params (DeltaSeconds :type Float%20%28single-precision%29))
  (bind _raycastoorigin (Variables|Default|GetRayCastoOrigin))
  (bind _returnvalue (Transformation|GetWorldLocation _raycastoorigin))
  (bind (_outhit _returnvalue_2) (Collision|LineTraceByChannel _returnvalue (+ _returnvalue (* (Math|Vector|GetForwardVector _raycastoorigin) (Variables|Default|GetDistance)) "0,0,-16.000000") "TraceTypeQuery1" false (Variables|Default|GetActors%20to%20Ignore) "None"))
  (if _returnvalue_2
    (Default|CallOnRaycastHit (.HitActor (Collision|BreakHitResult _outhit)))
    (Variables|Default|SetWasHit true)
    (elif (Variables|Default|GetWasHit)
      (Default|CallOnRaycastEnd))))