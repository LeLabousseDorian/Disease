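; First-person player character that handles look, movement, a pause menu and interaction with the world.
; Input arrives through player controller event dispatchers, which bind functions rebind to switch between default, holding, pushing and item-use states.
; A camera line trace picks up pickable components, toggles skeletal mesh animations or attaches push objects at a set walk speed.
; Picking up a teddy bear also enables use-item input, tied to a craziness-reduction event.
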(event EventBeginPlay
  (bind _returnvalue (UserInterface|CreateWidget "/Game/MyFolders/Blueprints/Widget/WBP_PauseMenu.WBP_PauseMenu_C"))
  (Variables|Default|SetPauseMenu _returnvalue)
  (Binds|DefaultLookBind)
  (Binds|DefaultMovementBind)
  (Binds|DefaultInteractBind)
  (Binds|DefaultPauseMenuBind))

(fn ConstructionScript)

(fn UpdatePostProcess
  (params (NewPostProcess :type Post%20Process%20Settings%20Structure))
  (Variables|/Script/Engine.CameraComponent|SetPostProcessSettings (Variables|MyCharacter|GetFirstPersonCamera) NewPostProcess))

(fn LookRight
  (params (AxisValue :type Float%20%28single-precision%29))
  (Pawn|Input|AddControllerYawInput (* AxisValue (Variables|Default|GetBaseTurnRate) (Utilities|Time|GetWorldDeltaSeconds))))

(fn LookUp
  (params (AxisValue :type Float%20%28single-precision%29))
  (Pawn|Input|AddControllerPitchInput (* AxisValue (Variables|Default|GetBaseLookUpRate) (Utilities|Time|GetWorldDeltaSeconds) (Variables|/Game/MyFolders/Blueprints/Player/BP_MyPlayerController.BP_MyPlayerController_C|GetTurnYAxisMultiplier (CallFunction|GetMyPlayerController)))))

(fn DefaultLookBind
  (bind _myplayercontroller (CallFunction|GetMyPlayerController))
  (EventDispatchers|UnbindallEventsfromOnLookRight _myplayercontroller)
  (EventDispatchers|UnbindallEventsfromOnLookUp _myplayercontroller)
  (EventDispatchers|BindEventtoOnLookRight _myplayercontroller (EventDispatchers|CreateEvent :!event LookRight))
  (EventDispatchers|BindEventtoOnLookUp _myplayercontroller (EventDispatchers|CreateEvent :!event LookUp)))

(fn MoveForward
  (params (AxisValue :type Float%20%28single-precision%29))
  (Pawn|Input|AddMovementInput (Math|Vector|GetForwardVector (Variables|MyCharacter|GetFirstPersonCamera)) AxisValue false))

(fn MoveRight
  (params (AxisValue :type Float%20%28single-precision%29))
  (Pawn|Input|AddMovementInput (Math|Vector|GetRightVector (Variables|MyCharacter|GetFirstPersonCamera)) AxisValue false))

(fn DefaultMovementBind
  (bind _myplayercontroller (CallFunction|GetMyPlayerController))
  (EventDispatchers|UnbindallEventsfromOnMoveForward _myplayercontroller)
  (EventDispatchers|UnbindallEventsfromOnMoveRight _myplayercontroller)
  (EventDispatchers|BindEventtoOnMoveForward _myplayercontroller (EventDispatchers|CreateEvent :!event MoveForward))
  (EventDispatchers|BindEventtoOnMoveRight _myplayercontroller (EventDispatchers|CreateEvent :!event MoveRight)))

(fn ChangeActorHeld
  (Default|OnPickup (Variables|ObjectHeld|GetAH_PickableComponent) (Variables|ObjectHeld|GetAH_StaticMeshComponent))
  (Transformation|AttachComponentToComponent (Variables|ObjectHeld|GetAH_StaticMeshComponent) (Variables|Default|GetObjectHeld) "None" "SnapToTarget" "SnapToTarget" "KeepRelative" true)
  (Transformation|SetWorldLocationAndRotation (Variables|ObjectHeld|GetAH_StaticMeshComponent) (+ (Variables|/Game/MyFolders/Blueprints/Components/BP_AC_Pickable.BP_AC_Pickable_C|GetLocation (Variables|ObjectHeld|GetAH_PickableComponent)) (Transformation|GetWorldLocation (Variables|Default|GetObjectHeld))) (Math|Rotator|CombineRotators (Variables|/Game/MyFolders/Blueprints/Components/BP_AC_Pickable.BP_AC_Pickable_C|GetRotation (Variables|ObjectHeld|GetAH_PickableComponent)) (Transformation|GetWorldRotation (Variables|Default|GetObjectHeld))) false false))

(fn SetObjectHeldVariables
  (params (NewActorHeld :type Actor%20Object%20Reference) (BP_SC_PickableComponent :type BP%20AC%20Pickable%20Object%20Reference) (HitComponent :type Primitive%20Component%20Object%20Reference))
  (Variables|ObjectHeld|SetActorHeld NewActorHeld)
  (Variables|ObjectHeld|SetAH_PickableComponent BP_SC_PickableComponent)
  (bind _asstatic_mesh_component (Utilities|Casting|CastToStaticMeshComponent HitComponent)
    (:then
      (Variables|ObjectHeld|SetAH_StaticMeshComponent _asstatic_mesh_component))
    (:CastFailed
      (Development|PrintString "Player.SetActorHeld : No Mesh Founded"))))

(fn HitPickable
  (params (Hit :type Hit%20Result%20Structure%20%28by%20ref%29))
  (bind (_bblockinghit _binitialoverlap _time _distance _location _impactpoint _normal _impactnormal _physmat _hitactor _hitcomponent) (Collision|BreakHitResult Hit))
  (bind _returnvalue (Actor|GetComponentbyClass _hitactor "/Game/MyFolders/Blueprints/Components/BP_AC_Pickable.BP_AC_Pickable_C"))
  ;[1 1 1] Pick the actor with BP_AC_Pickable pointed and place it in the hand of the player, bind the event corresponding if it's a teddybear
  (bind _isnounours (CallFunction|IsNounours? _hitactor))
  (if _isnounours
    (Binds|DefaultUseItemBind))
  (Utilities|IsValid _returnvalue
    (:Is%20Valid
      (Action|SetObjectHeldVariables _hitactor _returnvalue _hitcomponent)
      (Action|ChangeActorHeld)
      (Binds|PickableActorHeldBind))
    (:Is%20Not%20Valid
      (Development|PrintString "Player.HitPickable : No BP_AC_Pickable"))))

(fn HitSkeletalMesh
  (params (Hit :type Hit%20Result%20Structure%20%28by%20ref%29))
  ;[1 1 1] Play animation of SkeletalMesh Hit
  (bind _asskeletal_mesh_component (Utilities|Casting|CastToSkeletalMeshComponent (.HitComponent (Collision|BreakHitResult Hit)))
    (:then
      (Audio|Components|Audio|Play _asskeletal_mesh_component false)
      (Components|Timeline|SetPlayRate _asskeletal_mesh_component (* (Components|Animation|GetPlayRate _asskeletal_mesh_component) -1.0)))
    (:CastFailed
      (Development|PrintString "Player.HitSkeletalMesh : No SkeletalMeshComponent"))))

(fn HitPushObject
  (params (Hit :type Hit%20Result%20Structure%20%28by%20ref%29))
  (bind (_bblockinghit _binitialoverlap _time _distance _location _impactpoint _normal _impactnormal _physmat _hitactor _hitcomponent) (Collision|BreakHitResult Hit))
  (bind _asstatic_mesh_component (Utilities|Casting|CastToStaticMeshComponent _hitcomponent)
    (:then
      (Variables|Default|SetOH_StaticMeshComponent _asstatic_mesh_component)
      (Utilities|IsValid (Actor|GetComponentbyClass _hitactor "/Game/MyFolders/Blueprints/Components/BP_AC_PushObject.BP_AC_PushObject_C")
        (:Is%20Valid
          (Transformation|AttachComponentToComponent _hitcomponent (Variables|Default|GetObjectPush) "None" "KeepWorld" "KeepWorld" "KeepWorld" true)
          (Binds|PushActorHeldBind)
          (Variables|/Script/Engine.CharacterMovementComponent|SetMaxWalkSpeed (Variables|Character|GetCharacterMovement) (Variables|Default|GetMaxWalkSpeedPushingObject)))
        (:Is%20Not%20Valid
          (Development|PrintString "Player.HitPushObject : No BP_AC_PushObject"))))
    (:CastFailed
      (Development|PrintString "Player.HitPushObject : No Static Mesh"))))

(fn DefaultInteract
  (bind _firstpersoncamera (Variables|MyCharacter|GetFirstPersonCamera))
  (bind _returnvalue (Transformation|GetWorldLocation _firstpersoncamera))
  ;[1 1 1] Player has no item in hand
  (bind (_outhit _returnvalue_2) (Collision|LineTraceByChannel _returnvalue (+ _returnvalue (* (Math|Vector|GetForwardVector _firstpersoncamera) (Variables|Default|GetRayCastDistance)) "0,0,-16.000000") "TraceTypeQuery1" false 0 "None" true "(R=1.000000,G=0.000000,B=0.000000,A=1.000000)" "(R=0.000000,G=1.000000,B=0.000000,A=1.000000)" 2.0))
  (if _returnvalue_2
    (Utilities|FlowControl|Sequence
      (:then_0
        (Action|HitPickable _outhit))
      (:then_1
        (Action|HitSkeletalMesh _outhit))
      (:then_2
        (Action|HitPushObject _outhit)))
    (else
      (Development|PrintString "Player.DefaultInteract : Hit Nothing"))))

(fn DefaultInteractBind
  (bind _myplayercontroller (CallFunction|GetMyPlayerController))
  (EventDispatchers|UnbindallEventsfromOnInteractPressed _myplayercontroller)
  (EventDispatchers|UnbindallEventsfromOnInteractReleased _myplayercontroller)
  (EventDispatchers|UnbindallEventsfromOnUseItemPressed _myplayercontroller)
  (EventDispatchers|UnbindallEventsfromOnUseItemReleased _myplayercontroller)
  (EventDispatchers|BindEventtoOnInteractPressed _myplayercontroller (EventDispatchers|CreateEvent :!event DefaultInteract)))

(fn DefaultPauseMenuBind
  (bind _myplayercontroller (CallFunction|GetMyPlayerController))
  (EventDispatchers|UnbindallEventsfromOnStartPressed _myplayercontroller)
  (EventDispatchers|UnbindallEventsfromOnStartReleased _myplayercontroller)
  (EventDispatchers|BindEventtoOnStartPressed _myplayercontroller (EventDispatchers|CreateEvent :!event ShowPauseMenu))
  (EventDispatchers|BindEventtoOnStartReleased _myplayercontroller (EventDispatchers|CreateEvent :!event HidePauseMenu)))

(fn StopUsingItemBind
  (Binds|DefaultLookBind)
  (Binds|DefaultMovementBind))

(fn UsingItemBind
  (bind _myplayercontroller (CallFunction|GetMyPlayerController))
  (EventDispatchers|UnbindallEventsfromOnMoveForward _myplayercontroller)
  (EventDispatchers|UnbindallEventsfromOnMoveRight _myplayercontroller)
  (EventDispatchers|UnbindallEventsfromOnLookUp _myplayercontroller)
  (EventDispatchers|UnbindallEventsfromOnLookRight _myplayercontroller)
  (EventDispatchers|UnbindallEventsfromOnReduceCrazyness _myplayercontroller)
  (EventDispatchers|BindEventtoOnReduceCrazyness _myplayercontroller (EventDispatchers|CreateEvent _myplayercontroller :!event UsingTeddyBear)))

(fn DefaultUseItemBind
  (bind _myplayercontroller (CallFunction|GetMyPlayerController))
  (EventDispatchers|UnbindallEventsfromOnUseItemPressed _myplayercontroller)
  (EventDispatchers|UnbindallEventsfromOnUseItemReleased _myplayercontroller)
  (EventDispatchers|BindEventtoOnUseItemPressed _myplayercontroller (EventDispatchers|CreateEvent :!event UsingItemBind))
  (EventDispatchers|BindEventtoOnUseItemReleased _myplayercontroller (EventDispatchers|CreateEvent :!event StopUsingItemBind)))

(fn PickableActorHeldBind
  (bind _myplayercontroller (CallFunction|GetMyPlayerController))
  (EventDispatchers|UnbindallEventsfromOnInteractPressed _myplayercontroller)
  (EventDispatchers|BindEventtoOnInteractPressed _myplayercontroller (EventDispatchers|CreateEvent :!event DropPickableActor)))

(fn DropPickableActor
  (bind _ah_staticmeshcomponent (Variables|ObjectHeld|GetAH_StaticMeshComponent))
  ;[1 1 1] Player has pickable in hand
  (Default|OnDropDown (Variables|ObjectHeld|GetAH_PickableComponent) _ah_staticmeshcomponent)
  (Transformation|DetachFromComponent _ah_staticmeshcomponent "KeepWorld" "KeepWorld" "KeepWorld" true)
  (EventDispatchers|UnbindallEventsfromOnReduceCrazyness (CallFunction|GetMyPlayerController))
  (Binds|StopUsingItemBind)
  (Binds|DefaultInteractBind))

(fn DropPushActor
  ;[1 1 1] Player is pushing item
  (Binds|DefaultInteractBind)
  (Development|PrintString "Unbind UseItem")
  (Transformation|DetachFromComponent (Variables|Default|GetOH_StaticMeshComponent) "KeepWorld" "KeepWorld" "KeepWorld" true))

(fn PushActorHeldBind
  (bind _myplayercontroller (CallFunction|GetMyPlayerController))
  (EventDispatchers|UnbindallEventsfromOnInteractPressed _myplayercontroller)
  (EventDispatchers|BindEventtoOnInteractPressed _myplayercontroller (EventDispatchers|CreateEvent :!event DropPushActor)))

(fn IsNounours?
  (params (ActorHit :type Object%20Object%20Reference))
  (Utilities|Casting|CastToBP_TeddyBear ActorHit
    (:then
      (return true))
    (:CastFailed
      (return false))))

(fn ShowPauseMenu
  (UserInterface|Viewport|AddtoViewport (Variables|Default|GetPauseMenu) 0)
  (Game|SetGamePaused true)
  (Variables|/Script/Engine.PlayerController|SetbShowMouseCursor (Game|GetPlayerController 0) true))

(fn HidePauseMenu
  (Game|SetGamePaused false)
  (Widget|RemovefromParent (Variables|Default|GetPauseMenu))
  (Variables|/Script/Engine.PlayerController|SetbShowMouseCursor (Game|GetPlayerController 0) false))