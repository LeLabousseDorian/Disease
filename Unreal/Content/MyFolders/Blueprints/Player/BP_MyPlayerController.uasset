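; First-person player controller that handles object interaction and a rising "Crazyness" effect on BP_MyCharacter.
; Interact drops the held item or line-traces from the camera to attach pickables to the hand, attach pushables to a push point, and play skeletal mesh animations, reversing their play rate each hit.
; A Delay-throttled Tick adds delta time to capped Crazyness, which drives the character's post-process settings.
; A debug key flips the vertical turn multiplier.
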(event Custom|PostProcessTick
  (params (Value :type Float%20%28single-precision%29))
  ;[1 1 1] Add crazy value over time
  (CallFunction|AddCrazyness Value))

(event EventBeginPlay
  ;[1 0 0] Get the Player (need to change to an event system)
  (|GetPlayerRef))

(event Input|ActionEvents|InputActionInteract
  (params (Key :type Key%20Structure :default "None"))
  (bind _mycharacter (Variables|Character|GetMyCharacter))
  (bind _ah_staticmeshcomponent (Variables|ObjectHeld|GetAH_StaticMeshComponent))
  (bind _firstpersoncamera (Variables|/Game/MyFolders/Blueprints/Player/BP_MyCharacter.BP_MyCharacter_C|GetFirstPersonCamera _mycharacter))
  (bind _returnvalue (Transformation|GetWorldLocation _firstpersoncamera))
  ;[1 0 0] E Pressed
  (:Pressed
    (if (Utilities|IsValid (Variables|ObjectHeld|GetActorHeld))
      ;[1 1 1] Player has an item in hand
      (Default|OnDropDown (Variables|ObjectHeld|GetAH_PickableComponent) _ah_staticmeshcomponent)
      (Transformation|DetachFromComponent _ah_staticmeshcomponent "KeepWorld" "KeepWorld" "KeepWorld" true)
      (Variables|ObjectHeld|SetActorHeld 0)
      (else
        ;[1 1 1] Player has no item in hand
        (bind (_outhit _returnvalue_2) (Collision|LineTraceByChannel _returnvalue (+ _returnvalue (* (Math|Vector|GetForwardVector _firstpersoncamera) (Variables|Character|GetRayCastDistance)) "0,0,-16.000000") "TraceTypeQuery1" false 0 "Persistent" true "(R=1.000000,G=0.000000,B=0.000000,A=1.000000)" "(R=0.000000,G=1.000000,B=0.000000,A=1.000000)" 2.0))
        (if _returnvalue_2
          (Utilities|FlowControl|Sequence
            (:then_0
              (CallFunction|HitPickable _outhit))
            (:then_1
              (CallFunction|HitSkeletalMesh _outhit))
            (:then_2
              (Utilities|IsValid (Actor|GetComponentbyClass (.HitActor (Collision|BreakHitResult _outhit)) "/Game/MyFolders/Blueprints/Components/BP_AC_PushObject.BP_AC_PushObject_C")
                (:Is%20Valid
                  (Transformation|AttachComponentToComponent (.HitComponent (Collision|BreakHitResult _outhit)) (Variables|/Game/MyFolders/Blueprints/Player/BP_MyCharacter.BP_MyCharacter_C|GetObjectPush (Variables|Character|GetMyCharacter)) "None" "KeepWorld" "KeepWorld" "KeepWorld" true))
                (:Is%20Not%20Valid
                  (Development|PrintString "Controller.EventGraph : No BP_AC_PushObject")))))
          (else
            (Development|PrintString "Controller : Hit Nothing")))))))

(event Input|KeyboardEvents|F
  (params (Key :type Key%20Structure :default "None"))
  ;[1 0.2783 0] Debug : Invert Right Y Axis
  (:Pressed
    (CallFunction|SetTurnYAxisMultiplier (* (Variables|Character|GetTurnYAxisMultiplier) -1.0))))

(event EventTick
  (params (DeltaSeconds :type Float%20%28single-precision%29))
  (Utilities|FlowControl|Delay 0.1)
  (CallFunction|PostProcessTick DeltaSeconds))

(fn ConstructionScript)

(fn HitPickable
  (params (Hit :type Hit%20Result%20Structure%20%28by%20ref%29))
  (bind (_bblockinghit _binitialoverlap _time _distance _location _impactpoint _normal _impactnormal _physmat _hitactor _hitcomponent) (Collision|BreakHitResult Hit))
  (bind _returnvalue (Actor|GetComponentbyClass _hitactor "/Game/MyFolders/Blueprints/Components/BP_AC_Pickable.BP_AC_Pickable_C"))
  ;[1 1 1] Pick the actor with BP_AC_Pickable pointed and place it in the hand of the player
  (Utilities|IsValid _returnvalue
    (:Is%20Valid
      (CallFunction|SetObjectHeldVariables _hitactor _returnvalue _hitcomponent)
      (CallFunction|ChangeActorHeld))
    (:Is%20Not%20Valid
      (Development|PrintString "Controller.HitPickable : No BP_AC_Pickable"))))

(fn HitSkeletalMesh
  (params (Hit :type Hit%20Result%20Structure%20%28by%20ref%29))
  ;[1 1 1] Play animation of SkeletalMesh Hit
  (bind _asskeletal_mesh_component (Utilities|Casting|CastToSkeletalMeshComponent (.HitComponent (Collision|BreakHitResult Hit)))
    (:then
      (Audio|Components|Audio|Play _asskeletal_mesh_component false)
      (Components|Timeline|SetPlayRate _asskeletal_mesh_component (* (Components|Animation|GetPlayRate _asskeletal_mesh_component) -1.0)))
    (:CastFailed
      (Development|PrintString "No SkeletalMeshComponent"))))

(fn SetObjectHeldVariables
  (params (NewActorHeld :type Actor%20Object%20Reference) (BP_SC_PickableComponent :type BP%20AC%20Pickable%20Object%20Reference) (HitComponent :type Primitive%20Component%20Object%20Reference))
  (Variables|ObjectHeld|SetActorHeld NewActorHeld)
  (Variables|ObjectHeld|SetAH_PickableComponent BP_SC_PickableComponent)
  (bind _asstatic_mesh_component (Utilities|Casting|CastToStaticMeshComponent HitComponent)
    (:then
      (Variables|ObjectHeld|SetAH_StaticMeshComponent _asstatic_mesh_component))
    (:CastFailed
      (Development|PrintString "Controller.SetActorHeld : No Mesh Founded"))))

(fn ChangeActorHeld
  (Default|OnPickup (Variables|ObjectHeld|GetAH_PickableComponent) (Variables|ObjectHeld|GetAH_StaticMeshComponent))
  (Transformation|AttachComponentToComponent (Variables|ObjectHeld|GetAH_StaticMeshComponent) (Variables|/Game/MyFolders/Blueprints/Player/BP_MyCharacter.BP_MyCharacter_C|GetObjectHeld (Variables|Character|GetMyCharacter)) "None" "SnapToTarget" "SnapToTarget" "KeepRelative" true)
  (Transformation|SetWorldLocationAndRotation (Variables|ObjectHeld|GetAH_StaticMeshComponent) (+ (Variables|/Game/MyFolders/Blueprints/Components/BP_AC_Pickable.BP_AC_Pickable_C|GetLocation (Variables|ObjectHeld|GetAH_PickableComponent)) (Transformation|GetWorldLocation (Variables|/Game/MyFolders/Blueprints/Player/BP_MyCharacter.BP_MyCharacter_C|GetObjectHeld (Variables|Character|GetMyCharacter)))) (Math|Rotator|CombineRotators (Variables|/Game/MyFolders/Blueprints/Components/BP_AC_Pickable.BP_AC_Pickable_C|GetRotation (Variables|ObjectHeld|GetAH_PickableComponent)) (Transformation|GetWorldRotation (Variables|/Game/MyFolders/Blueprints/Player/BP_MyCharacter.BP_MyCharacter_C|GetFirstPersonCamera (Variables|Character|GetMyCharacter)))) false false)
  (Variables|Character|SetIsHolding true))

(fn AddCrazyness
  (params (Value :type Float%20%28single-precision%29))
  (if (>= (+ Value (Variables|Character|GetCrazyness)) 3.0)
    (Variables|Character|SetCrazyness 3.0)
    (else
      (Variables|Character|SetCrazyness (+ Value (Variables|Character|GetCrazyness)))))
  (CallFunction|UpdatePostProcess))

(fn UpdatePostProcess
  (bind _output_get (Variables|Character|SetPostProcessSettings (Utilities|Struct|MakePostProcessSettings (Variables|Character|GetCrazyness))))
  (Default|UpdatePostProcess (Variables|Character|GetMyCharacter) _output_get))

(fn SetTurnYAxisMultiplier
  (params (TurnYAxisMultiplier :type Float%20%28single-precision%29))
  (Variables|Character|SetTurnYAxisMultiplier TurnYAxisMultiplier))