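; First-person player Blueprint handling look, movement, pause menu, crazyness-driven camera post-process and object interaction.
; It binds its functions to player controller event dispatchers, rebinding Interact while an actor is held or pushed.
; A camera line trace drives interface-based pickup, looting, opening and pushing; held items can be used.
; An overlap collision shows the hand widget, and Veilleuse area events halve or restore the crazyness-over-time multiplier.
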(event OnComponentBeginOverlap(HandUICollision)
  (params (OverlappedComponent :type Primitive%20Component%20Object%20Reference) (OtherActor :type Actor%20Object%20Reference) (OtherComp :type Primitive%20Component%20Object%20Reference) (OtherBodyIndex :type Integer) (bFromSweep :type Boolean) (SweepResult :type Hit%20Result%20Structure%20%28by%20ref%29))
  (if (not (Widget|IsVisible (Variables|Default|GetHandWidget)))
    (if (Math|Boolean|ORBoolean (Utilities|DoesObjectImplementInterface OtherActor "/Game/MyFolders/Blueprints/Interface/BPI_ActorPickable.BPI_ActorPickable_C") (Utilities|DoesObjectImplementInterface OtherActor "/Game/MyFolders/Blueprints/Interface/BPI_Interactable.BPI_Interactable_C") (Utilities|DoesObjectImplementInterface OtherActor "/Game/MyFolders/Blueprints/Interface/BPI_Lootable.BPI_Lootable_C") (Utilities|DoesObjectImplementInterface OtherActor "/Game/MyFolders/Blueprints/Interface/BPI_OpenLocked.BPI_OpenLocked_C") (Utilities|DoesObjectImplementInterface OtherActor "/Game/MyFolders/Blueprints/Interface/BPI_PushableActor.BPI_PushableActor_C"))
      (UserInterface|Viewport|AddtoViewport (Variables|Default|GetHandWidget) 0))))

(event OnComponentEndOverlap(HandUICollision)
  (params (OverlappedComponent :type Primitive%20Component%20Object%20Reference) (OtherActor :type Actor%20Object%20Reference) (OtherComp :type Primitive%20Component%20Object%20Reference) (OtherBodyIndex :type Integer))
  (if (not (Collision|IsOverlappingActor (Variables|Default|GetHandUICollision) 0 :!class /Script/Engine.PrimitiveComponent))
    (Widget|RemovefromParent (Variables|Default|GetHandWidget))))

(event EventBeginPlay
  (Utilities|FlowControl|Sequence
    (:then_0
      ;[1 1 1] Pause Menu Widget
      (bind _returnvalue (UserInterface|CreateWidget "/Game/MyFolders/UI/WBP_PauseMenu.WBP_PauseMenu_C"))
      (Variables|Default|SetPauseMenu _returnvalue)
      (bind _returnvalue_2 (UserInterface|CreateWidget "/Game/MyFolders/UI/WBP_Grab.WBP_Grab_C"))
      (Variables|Default|SetHandWidget _returnvalue_2))
    (:then_1
      ;[1 1 1] Default Bind for the player
      (Binds|DefaultLookBind)
      (Binds|DefaultMovementBind)
      (Binds|DefaultInteractBind)
      (Binds|DefaultPauseMenuBind)
      (Binds|DefaultUpdatePostProcessBind)
      (Binds|DefaultUseItemBind))))

(event EventOnLowerMulitplier
  (bind _myplayercontroller (CallFunction|GetMyPlayerController))
  ;[1 1 1] When entering the Veilleuse AoE the crazyness multiplier
  (Variables|/Game/MyFolders/Blueprints/Player/BP_MyPlayerController.BP_MyPlayerController_C|SetAddedCrazynessOverTimeMultiplier _myplayercontroller (* (Variables|/Game/MyFolders/Blueprints/Player/BP_MyPlayerController.BP_MyPlayerController_C|GetAddedCrazynessOverTimeMultiplier _myplayercontroller) 0.5)))

(event EventOnHigherMulitplier
  (bind _myplayercontroller (CallFunction|GetMyPlayerController))
  ;[1 1 1] When leaving the Veilleuse AoE the crazyness multiplier
  (Variables|/Game/MyFolders/Blueprints/Player/BP_MyPlayerController.BP_MyPlayerController_C|SetAddedCrazynessOverTimeMultiplier _myplayercontroller (* (Variables|/Game/MyFolders/Blueprints/Player/BP_MyPlayerController.BP_MyPlayerController_C|GetAddedCrazynessOverTimeMultiplier _myplayercontroller) 2.0)))

(fn ConstructionScript)

(fn UpdatePostProcess
  (params (Crazyness :type Float%20%28single-precision%29))
  (Variables|/Script/Engine.CameraComponent|SetPostProcessSettings (Variables|MyCharacter|GetFirstPersonCamera) (Utilities|Struct|MakePostProcessSettings Crazyness)))

(fn LookRight
  (params (AxisValue :type Float%20%28single-precision%29))
  (Pawn|Input|AddControllerYawInput (* AxisValue (Variables|Default|GetBaseTurnRate) (Utilities|Time|GetWorldDeltaSeconds))))

(fn LookUp
  (params (AxisValue :type Float%20%28single-precision%29))
  (Pawn|Input|AddControllerPitchInput (* AxisValue (Variables|Default|GetBaseLookUpRate) (Utilities|Time|GetWorldDeltaSeconds) (Variables|/Game/MyFolders/Blueprints/Player/BP_MyPlayerController.BP_MyPlayerController_C|GetTurnYAxisMultiplier (CallFunction|GetMyPlayerController)))))

(fn DefaultLookBind
  (bind _myplayercontroller (CallFunction|GetMyPlayerController))
  (EventDispatchers|UnbindallEventsfromOnLookRight _myplayercontroller)
  (EventDispatchers|UnbindallEventsfromOnLookUp _myplayercontroller)
  (EventDispatchers|BindEventtoOnLookRight _myplayercontroller (EventDispatchers|CreateEvent :!event LookRight))
  (EventDispatchers|BindEventtoOnLookUp _myplayercontroller (EventDispatchers|CreateEvent :!event LookUp)))

(fn UnbindLook
  (bind _myplayercontroller (CallFunction|GetMyPlayerController))
  (EventDispatchers|UnbindallEventsfromOnLookRight _myplayercontroller)
  (EventDispatchers|UnbindallEventsfromOnLookUp _myplayercontroller))

(fn MoveForward
  (params (AxisValue :type Float%20%28single-precision%29))
  (Pawn|Input|AddMovementInput (Math|Vector|GetForwardVector (Variables|MyCharacter|GetFirstPersonCamera)) AxisValue false))

(fn MoveRight
  (params (AxisValue :type Float%20%28single-precision%29))
  (Pawn|Input|AddMovementInput (Math|Vector|GetRightVector (Variables|MyCharacter|GetFirstPersonCamera)) AxisValue false))

(fn DefaultMovementBind
  (bind _myplayercontroller (CallFunction|GetMyPlayerController))
  (EventDispatchers|UnbindallEventsfromOnMoveForward _myplayercontroller)
  (EventDispatchers|UnbindallEventsfromOnMoveRight _myplayercontroller)
  (EventDispatchers|BindEventtoOnMoveForward _myplayercontroller (EventDispatchers|CreateEvent :!event MoveForward))
  (EventDispatchers|BindEventtoOnMoveRight _myplayercontroller (EventDispatchers|CreateEvent :!event MoveRight)))

(fn DefaultInteract
  ;[1 1 1] Interact Input (no item) check what interface the actor implement
  (bind (_outhit _returnvalue) (CallFunction|CustomRaycast))
  (if _returnvalue
    (Utilities|FlowControl|Sequence
      (:then_0
        (Action|HitPickable _outhit)
        (Action|HitKey _outhit)
        (Action|HitSkeletalMesh _outhit)
        (Action|HitPushObject _outhit)))))

(fn HitPickable
  (params (Hit :type Hit%20Result%20Structure%20%28by%20ref%29))
  (bind _hitactor (Collision|BreakHitResult Hit))
  ;[1 1 1] If the actor hit implement the ActorPickable interface, then Attach it to the player
  (if (Utilities|DoesObjectImplementInterface _hitactor "/Game/MyFolders/Blueprints/Interface/BPI_ActorPickable.BPI_ActorPickable_C")
    (Class|BPIActorPickable|OnPickUp(Message) _hitactor)
    (bind _output_get (Variables|ObjectHeld|SetActorHeld _hitactor))
    (Transformation|AttachComponentToComponent _output_get (Variables|Default|GetObjectHeld) "None" "SnapToTarget" "SnapToTarget" "KeepRelative" true)
    (bind _offset (Class|BPIActorPickable|TransformOffset(Message) (Variables|ObjectHeld|GetActorHeld)))
    (Class|SceneComponent|AddLocalTransform (Variables|/Script/Engine.Actor|GetRootComponent (Variables|ObjectHeld|GetActorHeld)) _offset false false)
    (Binds|PickableActorHeldBind)))

(fn HitSkeletalMesh
  (params (Hit :type Hit%20Result%20Structure%20%28by%20ref%29))
  (bind (_bblockinghit _binitialoverlap _time _distance _location _impactpoint _normal _impactnormal _physmat _hitactor _hitcomponent) (Collision|BreakHitResult Hit))
  ;[1 1 1] Play animation of SkeletalMesh Hit
  (if (Utilities|DoesObjectImplementInterface _hitactor "/Game/MyFolders/Blueprints/Interface/BPI_OpenLocked.BPI_OpenLocked_C")
    (bind _canopen (Class|BPIOpenLocked|OnOpenLocked(Message) _hitactor self))
    (if _canopen
      (bind _asskeletal_mesh_component (Utilities|Casting|CastToSkeletalMeshComponent _hitcomponent :!label _label))
      (Audio|Components|Audio|Play _asskeletal_mesh_component false)
      (Components|Timeline|SetPlayRate _asskeletal_mesh_component (* (Components|Animation|GetPlayRate _asskeletal_mesh_component) -1.0)))
    (else
      (goto _label))))

(fn HitPushObject
  (params (Hit :type Hit%20Result%20Structure%20%28by%20ref%29))
  (bind _hitactor (Collision|BreakHitResult Hit))
  ;[1 1 1] If the actor implement the "Pushable Actor" Interface, then attach it to the player
  (if (Utilities|DoesObjectImplementInterface _hitactor "/Game/MyFolders/Blueprints/Interface/BPI_PushableActor.BPI_PushableActor_C")
    (Class|BPIPushableActor|OnPush(Message) _hitactor self)
    (bind _output_get (Variables|ObjectHeld|SetActorHeld _hitactor))
    (Transformation|AttachComponentToComponent _output_get (Variables|Default|GetObjectPush) "None" "KeepWorld" "KeepWorld" "KeepWorld" true)
    (Binds|PushActorHeldBind)))

(fn HitKey
  (params (Hit :type Hit%20Result%20Structure%20%28by%20ref%29))
  (bind _hitactor (Collision|BreakHitResult Hit))
  ;[1 1 1] If the actor hit implement the "Lootable" Interface
  (if (Utilities|DoesObjectImplementInterface _hitactor "/Game/MyFolders/Blueprints/Interface/BPI_Lootable.BPI_Lootable_C")
    (Class|BPILootable|OnLoot(Message) _hitactor self)))

(fn UnbindMovement
  (bind _myplayercontroller (CallFunction|GetMyPlayerController))
  (EventDispatchers|UnbindallEventsfromOnMoveForward _myplayercontroller)
  (EventDispatchers|UnbindallEventsfromOnMoveRight _myplayercontroller))

(fn DefaultInteractBind
  (bind _myplayercontroller (CallFunction|GetMyPlayerController))
  (EventDispatchers|UnbindallEventsfromOnInteractPressed _myplayercontroller)
  (EventDispatchers|UnbindallEventsfromOnInteractReleased _myplayercontroller)
  (EventDispatchers|BindEventtoOnInteractPressed _myplayercontroller (EventDispatchers|CreateEvent :!event DefaultInteract)))

(fn DefaultPauseMenuBind
  (bind _myplayercontroller (CallFunction|GetMyPlayerController))
  (EventDispatchers|UnbindallEventsfromOnStartPressed _myplayercontroller)
  (EventDispatchers|UnbindallEventsfromOnStartReleased _myplayercontroller)
  (EventDispatchers|BindEventtoOnStartPressed _myplayercontroller (EventDispatchers|CreateEvent :!event ShowPauseMenu))
  (EventDispatchers|BindEventtoOnStartReleased _myplayercontroller (EventDispatchers|CreateEvent :!event HidePauseMenu)))

(fn DefaultUpdatePostProcessBind
  (bind _myplayercontroller (CallFunction|GetMyPlayerController))
  (EventDispatchers|UnbindallEventsfromOnUpdatePostProcess _myplayercontroller)
  (EventDispatchers|BindEventtoOnUpdatePostProcess _myplayercontroller (EventDispatchers|CreateEvent :!event UpdatePostProcess)))

(fn DefaultUseItemBind
  (bind _myplayercontroller (CallFunction|GetMyPlayerController))
  (EventDispatchers|UnbindallEventsfromOnUseItemPressed _myplayercontroller)
  (EventDispatchers|UnbindallEventsfromOnUseItemReleased _myplayercontroller)
  (EventDispatchers|BindEventtoOnUseItemPressed _myplayercontroller (EventDispatchers|CreateEvent :!event UseItem))
  (EventDispatchers|BindEventtoOnUseItemReleased _myplayercontroller (EventDispatchers|CreateEvent :!event StopUsingItem)))

(fn PickableActorHeldBind
  (bind _myplayercontroller (CallFunction|GetMyPlayerController))
  (EventDispatchers|UnbindallEventsfromOnInteractPressed _myplayercontroller)
  (EventDispatchers|BindEventtoOnInteractPressed _myplayercontroller (EventDispatchers|CreateEvent :!event DropPickableActor)))

(fn DropPickableActor
  ;[1 1 1] Player drop the actor he's holding (call "on stop using" before dropping the item to avoid bug)
  (Transformation|DetachFromActor (Variables|ObjectHeld|GetActorHeld) "KeepWorld" "KeepWorld" "KeepWorld")
  (Class|BPIItemUsable|OnStopUsing(Message) (Variables|ObjectHeld|GetActorHeld) 0 self)
  (Class|BPIActorPickable|OnDropDown(Message) (Variables|ObjectHeld|GetActorHeld))
  (Variables|ObjectHeld|SetActorHeld 0)
  (Binds|DefaultInteractBind))

(fn DropPushActor
  ;[1 1 1] Player is pushing an item
  (Binds|DefaultInteractBind)
  (Transformation|DetachFromActor (Variables|ObjectHeld|GetActorHeld) "KeepWorld" "KeepWorld" "KeepWorld")
  (Class|BPIPushableActor|OnDrop(Message) (Variables|ObjectHeld|GetActorHeld) self)
  (Variables|ObjectHeld|SetActorHeld 0)
  (Binds|DefaultInteractBind))

(fn PushActorHeldBind
  (bind _myplayercontroller (CallFunction|GetMyPlayerController))
  (EventDispatchers|UnbindallEventsfromOnInteractPressed _myplayercontroller)
  (EventDispatchers|BindEventtoOnInteractPressed _myplayercontroller (EventDispatchers|CreateEvent :!event DropPushActor)))

(fn ShowPauseMenu
  (UserInterface|Viewport|AddtoViewport (Variables|Default|GetPauseMenu) 0)
  (Game|SetGamePaused true)
  (Variables|/Script/Engine.PlayerController|SetbShowMouseCursor (Game|GetPlayerController 0) true))

(fn HidePauseMenu
  (Default|ClosePauseMenu (Variables|Default|GetPauseMenu)))

(fn CustomRaycast
  (bind _firstpersoncamera (Variables|MyCharacter|GetFirstPersonCamera))
  (bind _returnvalue (Transformation|GetWorldLocation _firstpersoncamera))
  (bind (_outhit _returnvalue_2) (Collision|LineTraceByChannel _returnvalue (+ _returnvalue (* (Math|Vector|GetForwardVector _firstpersoncamera) (Variables|Default|GetRayCastDistance)) "0,0,-16.000000") "TraceTypeQuery1" false 0 "None" true "(R=1.000000,G=0.000000,B=0.000000,A=1.000000)" "(R=0.000000,G=1.000000,B=0.000000,A=1.000000)" 2.0))
  (return _outhit _returnvalue_2))

(fn UseItem
  (bind _actorheld (Variables|ObjectHeld|GetActorHeld))
  ;[1 1 1] Use the interface "ItemUsable" of the item held
  (if (Utilities|DoesObjectImplementInterface _actorheld "/Game/MyFolders/Blueprints/Interface/BPI_ItemUsable.BPI_ItemUsable_C")
    (Class|BPIItemUsable|OnStartUsing(Message) _actorheld (CallFunction|GetMyPlayerController) self)))

(fn StopUsingItem
  (bind _actorheld (Variables|ObjectHeld|GetActorHeld))
  ;[1 1 1] Use the interface "ItemUsable" of the item held
  (if (Utilities|DoesObjectImplementInterface _actorheld "/Game/MyFolders/Blueprints/Interface/BPI_ItemUsable.BPI_ItemUsable_C")
    (Class|BPIItemUsable|OnStopUsing(Message) _actorheld (CallFunction|GetMyPlayerController) self)))