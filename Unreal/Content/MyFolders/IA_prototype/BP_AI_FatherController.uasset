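; AI controller for the Father character, which runs BT_Father on the BB_Father blackboard.
; On BeginPlay it stores the player character in the blackboard and starts the behavior tree.
; A Delay on Tick acts as a repeating 30-second timer that sets ChangingRoom and writes a random RoomsLocation entry to RandomRoomLoc.
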(event EventTick
  (params (DeltaSeconds :type Float%20%28single-precision%29))
  (Utilities|FlowControl|Delay 3e+01)
  (AI|Components|Blackboard|SetValueasBool (Variables|Default|GetBlackboard%20Component) (Utilities|Name|MakeLiteralName "ChangingRoom") true)
  (AI|Components|Blackboard|SetValueasVector (Variables|Default|GetBlackboard%20Component) (Utilities|Name|MakeLiteralName "RandomRoomLoc") (Utilities|Array|Get(acopy) (Variables|Default|GetRoomsLocation) (Math|Random|RandomInteger (Utilities|Array|Length (Variables|Default|GetRoomsLocation))))))

(event EventBeginPlay
  (bind _blackboardcomponent (Class|AIController|UseBlackboard "/Game/MyFolders/IA_prototype/BB_Father.BB_Father"))
  (bind _output_get (Variables|Default|SetBlackboard%20Component _blackboardcomponent))
  (AI|Components|Blackboard|SetValueasObject _output_get (Utilities|Name|MakeLiteralName "Player") (Game|GetPlayerCharacter 0))
  (AI|RunBehaviorTree "/Game/MyFolders/IA_prototype/BT_Father.BT_Father"))

(fn ConstructionScript)