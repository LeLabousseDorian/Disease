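; BP_Father is a prototype AI-controlled pawn that reports whether it currently sees another pawn to its controller's Blackboard.
; On BeginPlay it caches the Blackboard and sets the CanSee key to false.
; PawnSensing sightings set CanSee to true, and a short retriggerable delay clears it once sightings stop, acting as a sight timeout.
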(event OnSeePawn(PawnSensing)
  (params (Pawn :type Pawn%20Object%20Reference))
  (AI|Components|Blackboard|SetValueasBool (Variables|Default|GetMyBlackboard) (Utilities|Name|MakeLiteralName "CanSee") true)
  (Utilities|FlowControl|RetriggerableDelay 0.6)
  (AI|Components|Blackboard|SetValueasBool (Variables|Default|GetMyBlackboard) (Utilities|Name|MakeLiteralName "CanSee") false))

(event EventBeginPlay
  (bind _output_get (Variables|Default|SetMyBlackboard (AI|GetBlackboard (Pawn|GetController))))
  (AI|Components|Blackboard|SetValueasBool _output_get (Utilities|Name|MakeLiteralName "CanSee") false))

(fn ConstructionScript)