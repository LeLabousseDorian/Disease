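; BP_IA_Prototype is a prototype AI pawn that roams randomly, then chases BP_MyCharacter when it sees it.
; Pawn Sensing starts the chase and plays an alert sound, rearmed by a retriggerable delay once sightings pause.
; Tick drives delayed roaming to random reachable points until a chase starts; IsChasing is never cleared, so roaming does not resume.
; CanSeeEnemy expires shortly after sight is lost, but its Tick check triggers nothing.
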(event OnSeePawn(PawnSensing)
  (params (Pawn :type Pawn%20Object%20Reference))
  ;[1 1 1] AI Chasing, Roaming and Audio
  (bind _asbp_my_character (Utilities|Casting|CastToBP_MyCharacter Pawn))
  (Utilities|FlowControl|Sequence
    (:then_0
      (Utilities|FlowControl|Sequence
        (:then_0
          (Variables|Default|SetCan%20See%20Enemy%20? true)
          (Variables|Default|SetIsChasing%20? true)
          (AI|AIMoveTo self "0, 0, 0" _asbp_my_character 5.0 false))
        (:then_1
          (Utilities|FlowControl|RetriggerableDelay 0.6)
          (Variables|Default|SetCan%20See%20Enemy%20? false))))
    (:then_1
      (Utilities|FlowControl|Sequence
        (:then_0
          (Utilities|FlowControl|DoOnce false :!label _label
            (:Completed
              (Audio|PlaySoundatLocation 0 (Transformation|GetActorLocation) "0, 0, 0" 1.0 1.0 0.0 0 0 0))))
        (:then_1
          (Utilities|FlowControl|RetriggerableDelay 1.0)
          (goto _label Reset))))))

(event EventTick
  (params (DeltaSeconds :type Float%20%28single-precision%29))
  ;[1 1 1] AI Chasing, Roaming and Audio
  (Utilities|FlowControl|Sequence
    (:then_0
      (if (Variables|Default|GetCan%20See%20Enemy%20?)
        (Utilities|FlowControl|Delay 0.4)
        (if (Variables|Default|GetCan%20See%20Enemy%20?)
          _)))
    (:then_1
      (if (not (Variables|Default|GetIsChasing%20?))
        (Utilities|FlowControl|Delay (Math|Random|RandomFloatinRange 2.0 5.0))
        (AI|AIMoveTo self (.RandomLocation (AI|Navigation|GetRandomReachablePointinRadius (Transformation|GetActorLocation) 1.5e+03 0 0)) 0 5.0 false)))))

(fn ConstructionScript)